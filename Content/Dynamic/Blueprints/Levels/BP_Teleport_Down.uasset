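; Level teleport trigger that moves a BP_Character to another point in the level when it enters the Box.
; On overlap, the character snaps without sweep to the location and rotation of the referenced NextPositionActor.
; It then gets Eoli from the player controller and resets that character's SpringArm to a fixed world yaw, preserving pitch and roll.
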(event OnComponentBeginOverlap(Box)
  (params (OverlappedComponent :type Primitive%20Component%20Object%20Reference) (OtherActor :type Actor%20Object%20Reference) (OtherComp :type Primitive%20Component%20Object%20Reference) (OtherBodyIndex :type Integer) (bFromSweep :type Boolean) (SweepResult :type Hit%20Result%20Structure%20%28by%20ref%29))
  (bind _next_position_actor (Variables|Default|GetNext%20Position%20Actor))
  (bind _asbp_character (Utilities|Casting|CastToBP_Character OtherActor))
  (Transformation|SetActorLocation _asbp_character (Transformation|GetActorLocation _next_position_actor) false true)
  (Transformation|SetActorRotation _asbp_character (Transformation|GetActorRotation _next_position_actor) true)
  (bind _aspc_ruin_from_the_past (Utilities|Casting|CastToPC_RuinFromThePast (Game|GetPlayerController 0)))
  (bind _eoli (Default|GetEoli _aspc_ruin_from_the_past))
  (Transformation|SetWorldRotation (Variables|/Game/Dynamic/Blueprints/Characters/Companion/BP_Eoli.BP_Eoli_C|GetSpringArm _eoli) (Math|Rotator|MakeRotator (.roll (Transformation|GetWorldRotation (Variables|/Game/Dynamic/Blueprints/Characters/Companion/BP_Eoli.BP_Eoli_C|GetSpringArm _eoli))) (.pitch (Transformation|GetWorldRotation (Variables|/Game/Dynamic/Blueprints/Characters/Companion/BP_Eoli.BP_Eoli_C|GetSpringArm _eoli))) 9e+01) false false))

(fn ConstructionScript)