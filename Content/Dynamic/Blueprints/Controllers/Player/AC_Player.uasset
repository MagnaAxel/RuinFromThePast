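; Player controller component that turns Enhanced Input actions into walk, jump and dash actions on its owning actor.
; On BeginPlay it looks up the sibling AC_Walk, AC_Jump and AC_Dash components, caches them and prints an error for any that are missing.
; Input events forward to each component's Do call, with the walk value written to MovementInput first, so this component only routes input.
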(event EventBeginPlay
  (CallFunction|BindInputActions))

(event Input|EnhancedActionEvents|EnhancedInputActionIA_Walk
  (params (ActionValue :type Vector%202D%20Structure) (ElapsedSeconds :type Float%20%28double-precision%29) (TriggeredSeconds :type Float%20%28double-precision%29) (InputAction :type Input%20Action%20Object%20Reference :default "/Game/Dynamic/Blueprints/Controllers/Player/Input/InputActions/IA_Walk.IA_Walk"))
  (Variables|/Game/Dynamic/Blueprints/Actions/Instances/AC_Walk.AC_Walk_C|SetMovementInput (Variables|Default|GetWalk) ActionValue)
  (Default|Do (Variables|Default|GetWalk)))

(event Input|EnhancedActionEvents|EnhancedInputActionIA_Jump
  (params (ActionValue :type Boolean) (ElapsedSeconds :type Float%20%28double-precision%29) (TriggeredSeconds :type Float%20%28double-precision%29) (InputAction :type Input%20Action%20Object%20Reference :default "/Game/Dynamic/Blueprints/Controllers/Player/Input/InputActions/IA_Jump.IA_Jump"))
  (Default|Do (Variables|Default|GetJump)))

(event Input|EnhancedActionEvents|EnhancedInputActionIA_Dash
  (params (ActionValue :type Boolean) (ElapsedSeconds :type Float%20%28double-precision%29) (TriggeredSeconds :type Float%20%28double-precision%29) (InputAction :type Input%20Action%20Object%20Reference :default "/Game/Dynamic/Blueprints/Controllers/Player/Input/InputActions/IA_Dash.IA_Dash"))
  (Default|Do (Variables|Default|GetDash)))

(fn BindInputActions
  (bind _returnvalue (Components|GetOwner))
  (bind _returnvalue_2 (Components|GetOwner))
  (bind _returnvalue_3 (Components|GetOwner))
  (bind _returnvalue_4 (Actor|GetComponentbyClass _returnvalue "/Game/Dynamic/Blueprints/Actions/Instances/AC_Dash.AC_Dash_C"))
  (bind _returnvalue_5 (Actor|GetComponentbyClass _returnvalue_2 "/Game/Dynamic/Blueprints/Actions/Instances/AC_Walk.AC_Walk_C"))
  (bind _returnvalue_6 (Actor|GetComponentbyClass _returnvalue_3 "/Game/Dynamic/Blueprints/Actions/Instances/AC_Jump.AC_Jump_C"))
  (Utilities|FlowControl|Sequence
    (:then_0
      (Utilities|IsValid _returnvalue_5
        (:Is%20Valid
          (Variables|Default|SetWalk _returnvalue_5))
        (:Is%20Not%20Valid
          (Development|PrintString "ERROR : No Walk Action found"))))
    (:then_1
      (Utilities|IsValid _returnvalue_6
        (:Is%20Valid
          (Variables|Default|SetJump _returnvalue_6))
        (:Is%20Not%20Valid
          (Development|PrintString "ERROR : No Jump Action found"))))
    (:then_2
      (Utilities|IsValid _returnvalue_4
        (:Is%20Valid
          (Variables|Default|SetDash _returnvalue_4))
        (:Is%20Not%20Valid
          (Development|PrintString "ERROR : No Dash Action found"))))))