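; PC_Default is the player controller that sets up the player's character, camera, input and HUD on BeginPlay.
; It finds the BP_Eoli actor in the level and possesses it, reporting through DevFeedback if none exists.
; It then adds player and combat-marker components to Eoli, attaches a spawned BP_PlayerCamera that keeps world rotation, registers IMC_Default, and creates the WI_Interface widget.
; Getters expose Eoli and the interface.
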(event EventBeginPlay
  (CallFunction|SetEoli)
  (CallFunction|AddPlayerComponents)
  (CallFunction|AddPlayerCamera)
  (CallFunction|AddPlayerController)
  (CallFunction|AddPlayerInterface))

(fn ConstructionScript)

(fn AddPlayerComponents
  (Game|AddComponentbyClass (Variables|Default|GetEoli) "/Game/Dynamic/Blueprints/Controllers/Player/AC_Player.AC_Player_C")
  (AddComponent|AddACCombatMarker (Variables|Default|GetEoli)))

(fn AddPlayerCamera
  (bind _returnvalue (Game|SpawnActorfromClass "/Game/Dynamic/Blueprints/Controllers/Player/Camera/BP_PlayerCamera.BP_PlayerCamera_C" (Transformation|GetActorTransform (Variables|Default|GetEoli)) "Undefined" "MultiplyWithRoot" 0 0))
  (Transformation|AttachActorToActor _returnvalue (Variables|Default|GetEoli) "None" "SnapToTarget" "KeepWorld" "KeepWorld" false))

(fn AddPlayerController
  (Input|AddMappingContext (PlayerController|LocalPlayerSubsystems|GetEnhancedInputLocalPlayerSubsystem self) "/Game/Dynamic/Blueprints/Controllers/Player/Input/IMC_Default.IMC_Default" 0 "(bIgnoreAllPressedKeysUntilRelease=True,bForceImmediately=False,bNotifyUserSettings=False)"))

(fn AddPlayerInterface
  (bind _returnvalue (UserInterface|CreateWidget "/Game/Dynamic/Blueprints/Controllers/Player/Interface/WI_Interface.WI_Interface_C" self))
  (bind _output_get (Variables|Default|SetInterface _returnvalue))
  (UserInterface|Viewport|AddtoViewport _output_get 0))

(fn GetInterface
  (return (Variables|Default|GetInterface)))

(fn SetEoli
  (bind _returnvalue (Actor|GetActorOfClass "/Game/Dynamic/Blueprints/Characters/Companion/BP_Eoli.BP_Eoli_C"))
  (Utilities|IsValid _returnvalue
    (:Is%20Valid
      (bind _output_get (Variables|Default|SetEoli _returnvalue))
      (Pawn|Possess _output_get))
    (:Is%20Not%20Valid
      (CallFunction|DevFeedback "NewEnumerator2" "Eoli Character not found"))))

(fn GetEoli
  (return (Variables|Default|GetEoli)))