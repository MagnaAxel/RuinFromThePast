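; Player controller for Ruin From The Past that possesses the level's BP_Eoli character and routes player input to it.
; On BeginPlay it adds player-only action components to Eoli, caches action and combat components by class, then sets up the input mapping, attached camera and HUD widget.
; Enhanced Input events forward to each component's TryAction, with Walk receiving the movement value and Previous/Next cycling the combat target.
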(event EventBeginPlay
  (CallFunction|SetEoli)
  (CallFunction|AddPlayerComponents)
  (CallFunction|BindInputActions)
  (CallFunction|AddPlayerMappingContext)
  (CallFunction|AddPlayerCamera)
  (CallFunction|AddPlayerInterface))

(event Input|EnhancedActionEvents|EnhancedInputActionIA_Walk
  (params (ActionValue :type Vector%202D%20Structure) (ElapsedSeconds :type Float%20%28double-precision%29) (TriggeredSeconds :type Float%20%28double-precision%29) (InputAction :type Input%20Action%20Object%20Reference :default "/Game/Dynamic/Blueprints/Controllers/Player/Input/InputActions/IA_Walk.IA_Walk"))
  (Variables|/Game/Dynamic/Blueprints/Actions/Instances/AC_Walk.AC_Walk_C|SetMovementInput (Variables|Default|GetWalk) ActionValue)
  (Default|TryAction (Variables|Default|GetWalk)))

(event Input|EnhancedActionEvents|EnhancedInputActionIA_Jump
  (params (ActionValue :type Boolean) (ElapsedSeconds :type Float%20%28double-precision%29) (TriggeredSeconds :type Float%20%28double-precision%29) (InputAction :type Input%20Action%20Object%20Reference :default "/Game/Dynamic/Blueprints/Controllers/Player/Input/InputActions/IA_Jump.IA_Jump"))
  (Default|TryAction (Variables|Default|GetJump)))

(event Input|EnhancedActionEvents|EnhancedInputActionIA_Dash
  (params (ActionValue :type Boolean) (ElapsedSeconds :type Float%20%28double-precision%29) (TriggeredSeconds :type Float%20%28double-precision%29) (InputAction :type Input%20Action%20Object%20Reference :default "/Game/Dynamic/Blueprints/Controllers/Player/Input/InputActions/IA_Dash.IA_Dash"))
  (Default|TryAction (Variables|Default|GetDash)))

(event Input|EnhancedActionEvents|EnhancedInputActionIA_Interact
  (params (ActionValue :type Boolean) (ElapsedSeconds :type Float%20%28double-precision%29) (TriggeredSeconds :type Float%20%28double-precision%29) (InputAction :type Input%20Action%20Object%20Reference :default "/Game/Dynamic/Blueprints/Controllers/Player/Input/InputActions/IA_Interact.IA_Interact"))
  (Default|TryAction (Variables|Default|GetInteract)))

(event Input|EnhancedActionEvents|EnhancedInputActionIA_Attack
  (params (ActionValue :type Boolean) (ElapsedSeconds :type Float%20%28double-precision%29) (TriggeredSeconds :type Float%20%28double-precision%29) (InputAction :type Input%20Action%20Object%20Reference :default "/Game/Dynamic/Blueprints/Controllers/Player/Input/InputActions/IA_Attack.IA_Attack"))
  (Default|TryAction (Variables|Default|GetAttack)))

(event Input|EnhancedActionEvents|EnhancedInputActionIA_Eat
  (params (ActionValue :type Boolean) (ElapsedSeconds :type Float%20%28double-precision%29) (TriggeredSeconds :type Float%20%28double-precision%29) (InputAction :type Input%20Action%20Object%20Reference :default "/Game/Dynamic/Blueprints/Controllers/Player/Input/InputActions/IA_Eat.IA_Eat"))
  (Default|TryAction (Variables|Default|GetEat)))

(event Input|EnhancedActionEvents|EnhancedInputActionIA_Previous
  (params (ActionValue :type Boolean) (ElapsedSeconds :type Float%20%28double-precision%29) (TriggeredSeconds :type Float%20%28double-precision%29) (InputAction :type Input%20Action%20Object%20Reference :default "/Game/Dynamic/Blueprints/Controllers/Player/Input/InputActions/IA_Previous.IA_Previous"))
  (Default|PreviousTargetIndex (Variables|Default|GetCombat)))

(event Input|EnhancedActionEvents|EnhancedInputActionIA_Next
  (params (ActionValue :type Boolean) (ElapsedSeconds :type Float%20%28double-precision%29) (TriggeredSeconds :type Float%20%28double-precision%29) (InputAction :type Input%20Action%20Object%20Reference :default "/Game/Dynamic/Blueprints/Controllers/Player/Input/InputActions/IA_Next.IA_Next"))
  (Default|NextTargetIndex (Variables|Default|GetCombat)))

(fn ConstructionScript)

(fn AddPlayerComponents
  (AddComponent|AddACJump (Variables|Default|GetEoli))
  (AddComponent|AddACDash (Variables|Default|GetEoli))
  (AddComponent|AddACEat (Variables|Default|GetEoli))
  (AddComponent|AddACInteract (Variables|Default|GetEoli))
  (AddComponent|AddACCombatMarker (Variables|Default|GetEoli))
  (AddComponent|AddACInventory (Variables|Default|GetEoli))
  (AddComponent|AddACLocket (Variables|Default|GetEoli)))

(fn BindInputActions
  (bind _eoli (Variables|Default|GetEoli))
  (bind _eoli_2 (Variables|Default|GetEoli))
  (bind _eoli_3 (Variables|Default|GetEoli))
  (bind _eoli_4 (Variables|Default|GetEoli))
  (bind _eoli_5 (Variables|Default|GetEoli))
  (bind _eoli_6 (Variables|Default|GetEoli))
  (bind _eoli_7 (Variables|Default|GetEoli))
  (bind _returnvalue (Actor|GetComponentbyClass _eoli_4 "/Game/Dynamic/Blueprints/Actions/Instances/AC_Dash.AC_Dash_C"))
  (bind _returnvalue_2 (Actor|GetComponentbyClass _eoli_2 "/Game/Dynamic/Blueprints/Actions/Instances/AC_Walk.AC_Walk_C"))
  (bind _returnvalue_3 (Actor|GetComponentbyClass _eoli_5 "/Game/Dynamic/Blueprints/Actions/Instances/Interact/AC_Interact.AC_Interact_C"))
  (bind _returnvalue_4 (Actor|GetComponentbyClass _eoli_6 "/Game/Dynamic/Blueprints/Actions/Instances/AC_Attack.AC_Attack_C"))
  (bind _returnvalue_5 (Actor|GetComponentbyClass _eoli_7 "/Game/Dynamic/Blueprints/Actions/Instances/AC_Eat.AC_Eat_C"))
  (bind _returnvalue_6 (Actor|GetComponentbyClass _eoli "/Game/Dynamic/Blueprints/Combat/AC_Combat.AC_Combat_C"))
  (bind _returnvalue_7 (Actor|GetComponentbyClass _eoli_3 "/Game/Dynamic/Blueprints/Actions/Instances/AC_Jump.AC_Jump_C"))
  (Utilities|FlowControl|Sequence
    (:then_0
      (Utilities|IsValid _returnvalue_2
        (:Is%20Valid
          (Variables|Default|SetWalk _returnvalue_2))
        (:Is%20Not%20Valid
          (Development|PrintString "ERROR : No Walk Action found" true true "(R=1.000000,G=0.000000,B=0.000000,A=1.000000)"))))
    (:then_1
      (Utilities|IsValid _returnvalue_7
        (:Is%20Valid
          (Variables|Default|SetJump _returnvalue_7))
        (:Is%20Not%20Valid
          (Development|PrintString "ERROR : No Jump Action found" true true "(R=1.000000,G=0.000000,B=0.000000,A=1.000000)"))))
    (:then_2
      (Utilities|IsValid _returnvalue
        (:Is%20Valid
          (Variables|Default|SetDash _returnvalue))
        (:Is%20Not%20Valid
          (Development|PrintString "ERROR : No Dash Action found" true true "(R=1.000000,G=0.000000,B=0.000000,A=1.000000)"))))
    (:then_3
      (Utilities|IsValid _returnvalue_3
        (:Is%20Valid
          (Variables|Default|SetInteract _returnvalue_3))
        (:Is%20Not%20Valid
          (Development|PrintString "ERROR : No Interact Action found" true true "(R=1.000000,G=0.000000,B=0.000000,A=1.000000)"))))
    (:then_4
      (Utilities|IsValid _returnvalue_4
        (:Is%20Valid
          (Variables|Default|SetAttack _returnvalue_4))
        (:Is%20Not%20Valid
          (Development|PrintString "ERROR : No Attack Action found" true true "(R=1.000000,G=0.000000,B=0.000000,A=1.000000)"))))
    (:then_5
      (Utilities|IsValid _returnvalue_5
        (:Is%20Valid
          (Variables|Default|SetEat _returnvalue_5))
        (:Is%20Not%20Valid
          (Development|PrintString "ERROR : No Eat Action found" true true "(R=1.000000,G=0.000000,B=0.000000,A=1.000000)"))))
    (:then_6
      (Utilities|IsValid _returnvalue_6
        (:Is%20Valid
          (Variables|Default|SetCombat _returnvalue_6))
        (:Is%20Not%20Valid
          (Development|PrintString "ERROR : No Combat Component found" true true "(R=1.000000,G=0.000000,B=0.000000,A=1.000000)"))))))

(fn AddPlayerCamera
  (bind _returnvalue (Game|SpawnActorfromClass "/Game/Dynamic/Blueprints/Controllers/Player/Camera/BP_PlayerCamera.BP_PlayerCamera_C" (Transformation|GetActorTransform (Variables|Default|GetEoli)) "Undefined" "MultiplyWithRoot" 0 0))
  (Transformation|AttachActorToActor _returnvalue (Variables|Default|GetEoli) "None" "SnapToTarget" "KeepWorld" "KeepWorld" false))

(fn AddPlayerMappingContext
  (Input|AddMappingContext (PlayerController|LocalPlayerSubsystems|GetEnhancedInputLocalPlayerSubsystem self) "/Game/Dynamic/Blueprints/Controllers/Player/Input/IMC_Default.IMC_Default" 0 "(bIgnoreAllPressedKeysUntilRelease=True,bForceImmediately=False,bNotifyUserSettings=False)"))

(fn AddPlayerInterface
  (bind _returnvalue (UserInterface|CreateWidget "/Game/Dynamic/Blueprints/Controllers/Player/Interface/WI_RuinFromThePast.WI_RuinFromThePast_C" self))
  (bind _output_get (Variables|Default|SetWI _returnvalue))
  (UserInterface|Viewport|AddtoViewport _output_get 0))

(fn GetWI
  (return (Variables|Default|GetWI)))

(fn SetEoli
  (bind _returnvalue (Actor|GetActorOfClass "/Game/Dynamic/Blueprints/Characters/Companion/BP_Eoli.BP_Eoli_C"))
  (Utilities|IsValid _returnvalue
    (:Is%20Valid
      (bind _output_get (Variables|Default|SetEoli _returnvalue))
      (Pawn|Possess _output_get))
    (:Is%20Not%20Valid
      (CallFunction|DevFeedback "NewEnumerator2" "Eoli Character not found"))))

(fn GetEoli
  (return (Variables|Default|GetEoli)))