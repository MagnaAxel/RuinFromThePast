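; Player camera actor that switches a spring arm between an exploration view and a combat view.
; After a one-tick delay, it binds to the AC_Combat component on its attach parent and starts in exploration view.
; Combat enter and leave events trigger a timeline that lerps arm length and pitch from current values to the target view.
; The start pitch is read in world space but applied as relative rotation.
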(event Custom|EntersCombat_Event
  (CallFunction|SetCombatView))

(event Custom|LeavesCombat_Event
  (CallFunction|SetExplorationView))

(event EventBeginPlay
  (bind _returnvalue (Actor|GetAttachParentActor))
  (bind _returnvalue_2 (Actor|GetComponentbyClass _returnvalue "/Game/Dynamic/Blueprints/Combat/AC_Combat.AC_Combat_C"))
  (Utilities|FlowControl|DelayUntilNextTick)
  (Utilities|IsValid _returnvalue_2
    (:Is%20Valid
      (EventDispatchers|AssignEntersCombat _returnvalue_2 (delegate Custom|EntersCombat_Event))
      (EventDispatchers|AssignLeavesCombat _returnvalue_2 (delegate Custom|LeavesCombat_Event))
      (CallFunction|SetExplorationView))
    (:Is%20Not%20Valid
      (Development|PrintString "ERROR : Combat component not found"))))

(event Custom|ViewTransition
  (params (StartDistance :type Float%20%28double-precision%29) (StartAngle :type Float%20%28double-precision%29) (EndDistance :type Float%20%28double-precision%29) (EndAngle :type Float%20%28double-precision%29))
  (bind _viewtransitiontrack (Timeline|ViewTransitionTimeline PlayFromStart)
    (:Update
      (Variables|/Script/Engine.SpringArmComponent|SetTargetArmLength (Variables|Default|GetSpringArm) (Math|Float|Lerp StartDistance EndDistance _viewtransitiontrack))
      (Transformation|SetRelativeRotation (Variables|Default|GetSpringArm) (Math|Rotator|MakeRotator 0.0 (Math|Float|Lerp StartAngle EndAngle _viewtransitiontrack) 0.0) false false))))

(fn ConstructionScript)

(fn SetExplorationView
  (CallFunction|ViewTransition (Variables|/Script/Engine.SpringArmComponent|GetTargetArmLength (Variables|Default|GetSpringArm)) (.pitch (Transformation|GetWorldRotation (Variables|Default|GetSpringArm))) (Variables|Default|GetExplorationCameraDistance) (Variables|Default|GetExplorationCameraAngle)))

(fn SetCombatView
  (CallFunction|ViewTransition (Variables|/Script/Engine.SpringArmComponent|GetTargetArmLength (Variables|Default|GetSpringArm)) (.pitch (Transformation|GetWorldRotation (Variables|Default|GetSpringArm))) (Variables|Default|GetCombatDistance) (Variables|Default|GetCombatAngle)))