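; BP_ExplorationSquadStart marks where an exploration squad starts, with five capsule components as individual start spots.
; When an actor with an AC_Player component begins overlapping its Sphere, it registers itself as ExplorationSquadStart on the GSB game state, replacing any previous reference.
; GetOneStart maps an index to one of the five capsules.
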(event OnComponentBeginOverlap(Sphere)
  (params (OverlappedComponent :type Primitive%20Component%20Object%20Reference) (OtherActor :type Actor%20Object%20Reference) (OtherComp :type Primitive%20Component%20Object%20Reference) (OtherBodyIndex :type Integer) (bFromSweep :type Boolean) (SweepResult :type Hit%20Result%20Structure%20%28by%20ref%29))
  (Utilities|IsValid (Actor|GetComponentbyClass OtherActor "/Game/Dynamic/Blueprints/Controllers/Player/AC_Player.AC_Player_C")
    (:Is%20Valid
      (bind _asgsb (Utilities|Casting|CastToGSB (Game|GetGameState)))
      (Variables|/Game/Dynamic/Blueprints/Controllers/Player/GSB.GSB_C|SetExplorationSquadStart _asgsb self))))

(fn ConstructionScript)

(fn GetOneStart
  (params (Index :type Integer))
  (return (Utilities|Select :Index Index :Option%200 (Variables|Default|GetCapsule0) :Option%201 (Variables|Default|GetCapsule1) :Option%202 (Variables|Default|GetCapsule2) :Option%203 (Variables|Default|GetCapsule3) :Option%204 (Variables|Default|GetCapsule4))))