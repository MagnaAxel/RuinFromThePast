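; Actor component that manages its owner's Constitution, Resistance, Agility and Strength, along with health.
; UpdateStatistics sums base values, every AC_Accessory bonus and the AC_Exaltation bonus, floors them at zero and derives percentage factors.
; Constitution caps health, while Resistance subtracts a flat amount from incoming damage.
; SetHealth clamps, notifies of changes and starts a looping Constitution-scaled regeneration timer when wounded, clearing it only at zero health.
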(event EventBeginPlay
  (CallFunction|UpdateStatistics)
  (CallFunction|SetHealth (Variables|FinalStatistics|GetFinalConstitution)))

(event EventDamage
  (params (Damage :type Integer%20%28by%20ref%29))
  (CallFunction|SubstractHealth (- Damage (* 10 (Variables|StatisticFactors|GetResistanceFactor)))))

(event Custom|PlayRegeneration
  (bind _returnvalue (Utilities|Time|SetTimerbyEvent (delegate Custom|Regenerate) 1.0 true))
  (Variables|Default|SetRegenerationCooldown _returnvalue))

(event Custom|Regenerate
  (CallFunction|AddHealth (+ 1 (Variables|StatisticFactors|GetConstitutionFactor))))

(fn UpdateStatistics
  (bind _returnvalue (Components|GetOwner))
  (bind _returnvalue_2 (Actor|GetComponentbyClass _returnvalue "/Game/Dynamic/Blueprints/Exaltation/AC_Exaltation.AC_Exaltation_C"))
  (Utilities|FlowControl|Sequence
    (:then_0
      (LocalVariables|SetTemporaryConstitution (Variables|BaseStatistics|GetBaseConstitution))
      (LocalVariables|SetTemporaryResistance (Variables|BaseStatistics|GetBaseResistance))
      (LocalVariables|SetTemporaryAgility (Variables|BaseStatistics|GetBaseAgility))
      (LocalVariables|SetTemporaryStrength (Variables|BaseStatistics|GetBaseStrength)))
    (:then_1
      (for _array_element (Actor|GetComponentsByClass (Components|GetOwner) "/Game/Dynamic/Blueprints/Objects/Accessories/AC_Accessory.AC_Accessory_C")
        (bind _asbp_accessory (Default|GetAccessory _array_element))
        (Utilities|IsValid _asbp_accessory
          (:Is%20Valid
            (LocalVariables|SetTemporaryConstitution (+ (LocalVariables|GetTemporaryConstitution) (Variables|/Game/Dynamic/Blueprints/Objects/Accessories/BP_Accessory.BP_Accessory_C|GetConstitution _asbp_accessory)))
            (LocalVariables|SetTemporaryResistance (+ (LocalVariables|GetTemporaryResistance) (Variables|/Game/Dynamic/Blueprints/Objects/Accessories/BP_Accessory.BP_Accessory_C|GetResistance _asbp_accessory)))
            (LocalVariables|SetTemporaryAgility (+ (LocalVariables|GetTemporaryAgility) (Variables|/Game/Dynamic/Blueprints/Objects/Accessories/BP_Accessory.BP_Accessory_C|GetAgility _asbp_accessory)))
            (LocalVariables|SetTemporaryStrength (+ (LocalVariables|GetTemporaryStrength) (Variables|/Game/Dynamic/Blueprints/Objects/Accessories/BP_Accessory.BP_Accessory_C|GetStrength _asbp_accessory)))))))
    (:then_2
      (Utilities|IsValid _returnvalue_2
        (:Is%20Valid
          (bind _exaltation (Default|GetExaltation _returnvalue_2))
          (LocalVariables|SetTemporaryConstitution (+ (LocalVariables|GetTemporaryConstitution) _exaltation))
          (LocalVariables|SetTemporaryResistance (+ (LocalVariables|GetTemporaryResistance) _exaltation))
          (LocalVariables|SetTemporaryAgility (+ (LocalVariables|GetTemporaryAgility) _exaltation))
          (LocalVariables|SetTemporaryStrength (+ (LocalVariables|GetTemporaryStrength) _exaltation)))))
    (:then_3
      (Variables|FinalStatistics|SetFinalConstitution (Math|Integer|Max(Integer) (LocalVariables|GetTemporaryConstitution)))
      (Variables|FinalStatistics|SetFinalResistance (Math|Integer|Max(Integer) (LocalVariables|GetTemporaryResistance)))
      (Variables|FinalStatistics|SetFinalAgility (Math|Integer|Max(Integer) (LocalVariables|GetTemporaryAgility)))
      (Variables|FinalStatistics|SetFinalStrength (Math|Integer|Max(Integer) (LocalVariables|GetTemporaryStrength))))
    (:then_4
      (Variables|StatisticFactors|SetConstitutionFactor (* (Variables|FinalStatistics|GetFinalConstitution) 0.01))
      (Variables|StatisticFactors|SetResistanceFactor (* (Variables|FinalStatistics|GetFinalResistance) 0.01))
      (Variables|StatisticFactors|SetAgilityFactor (* (Variables|FinalStatistics|GetFinalAgility) 0.01))
      (Variables|StatisticFactors|SetStrengthFactor (* (Variables|FinalStatistics|GetFinalStrength) 0.01)))
    (:then_5
      (if (> (Variables|Default|GetHealth) (Variables|FinalStatistics|GetFinalConstitution))
        (CallFunction|SetHealth (Variables|FinalStatistics|GetFinalConstitution))))))

(fn SetHealth
  (params (Health :type Integer))
  (Utilities|FlowControl|Sequence
    (:then_0
      (Variables|Default|SetHealth (Math|Integer|Clamp(Integer) Health 0 (Variables|FinalStatistics|GetFinalConstitution)))
      (Default|CallHealthHasChanged))
    (:then_1
      (if (> (Variables|Default|GetHealth) 0)
        (if (< (Variables|Default|GetHealth) (Variables|FinalStatistics|GetFinalConstitution))
          (if (not (Utilities|Time|IsValidTimerHandle (Variables|Default|GetRegenerationCooldown)))
            (CallFunction|PlayRegeneration)))
        (else
          (Utilities|Time|ClearandInvalidateTimerbyHandle (Variables|Default|GetRegenerationCooldown)))))))

(fn GetHealth
  (return (Variables|Default|GetHealth)))

(fn AddHealth
  (params (Health :type Integer))
  (CallFunction|SetHealth (+ (Variables|Default|GetHealth) Health)))

(fn SubstractHealth
  (params (Health :type Integer))
  (CallFunction|SetHealth (- (Variables|Default|GetHealth) Health)))