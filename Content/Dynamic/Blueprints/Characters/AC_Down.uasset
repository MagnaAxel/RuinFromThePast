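; AC_Down is a character component that adds a downed state to BP_Character in place of death.
; While it is present it deactivates the character's ACDeath component, reactivating it on EndPlay.
; It listens to health changes from ACStatistic and calls Down at zero health.
; Down and Undown lock or unlock every AC_Action component on the owner and fire the matching Downs or Undowns dispatcher.
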(event Custom|ChangesHealth_Event
  (params (NewHealth :type Integer))
  (if (== NewHealth 0)
    (CallFunction|Down)))

(event EventBeginPlay
  (bind _asbp_character (Utilities|Casting|CastToBP_Character (Components|GetOwner)))
  (Components|Activation|Deactivate (Variables|/Game/Dynamic/Blueprints/Characters/BP_Character.BP_Character_C|GetAC_Death _asbp_character))
  (EventDispatchers|AssignChangesHealth (Variables|/Game/Dynamic/Blueprints/Characters/BP_Character.BP_Character_C|GetAC_Statistic _asbp_character) (delegate Custom|ChangesHealth_Event)))

(event EventEndPlay
  (params (EndPlayReason :type EEndPlayReason%20Enum :default "Destroyed"))
  (bind _asbp_character (Utilities|Casting|CastToBP_Character (Components|GetOwner)))
  (Components|Activation|Activate (Variables|/Game/Dynamic/Blueprints/Characters/BP_Character.BP_Character_C|GetAC_Death _asbp_character) false))

(fn Down
  (for _array_element (Actor|GetComponentsByClass (Components|GetOwner) "/Game/Dynamic/Blueprints/Actions/AC_Action.AC_Action_C")
    (Default|Lock _array_element))
  (Default|CallDowns))

(fn Undown
  (for _array_element (Actor|GetComponentsByClass (Components|GetOwner) "/Game/Dynamic/Blueprints/Actions/AC_Action.AC_Action_C")
    (Default|Unlock _array_element))
  (Default|CallUndowns))