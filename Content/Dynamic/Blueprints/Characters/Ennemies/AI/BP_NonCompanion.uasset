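; BP_NonCompanion is an enemy AI character with placeholder combat behavior.
; It exposes functions for attacking, patrol route, ideal range and movement speed; Attack only prints a message and ideal range returns zero.
; SetMovementSpeed maps a movement state to the CharacterMovement max walk speed.
; On BeginPlay it binds to the ACStatistic health-change dispatcher and destroys itself a tick after any health change, regardless of the new value.
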(event Custom|HealthHasChanged_Event
  (params (NewHealth :type Integer))
  (Utilities|FlowControl|DelayUntilNextTick)
  (Actor|DestroyActor))

(event Custom|Attack
  (Development|PrintString "Enemy Attack"))

(event EventBeginPlay
  (EventDispatchers|AssignChangesHealth (Variables|Default|GetAC_Statistic) (delegate Custom|HealthHasChanged_Event)))

(fn ConstructionScript)

(fn GetIdealRange
  (return 0.0))

(fn GetPatrolRoute
  (return (Variables|Default|GetPatrolRoute)))

(fn SetMovementSpeed
  (params (Speed :type EN_MovementSpeed%20Enum :default "NewEnumerator0"))
  (bind _output_get (Variables|/Script/Engine.CharacterMovementComponent|SetMaxWalkSpeed (Variables|Character|GetCharacterMovement) (Utilities|Select :Index Speed :NewEnumerator0 0.0 :NewEnumerator1 1e+02 :NewEnumerator2 3e+02 :NewEnumerator3 5e+02)))
  (return _output_get))