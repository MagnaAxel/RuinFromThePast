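; AC_Down is a character component that puts its BP_Character into a downed state when health reaches zero, in place of ACDeath.
; It deactivates ACDeath on BeginPlay, listens to ACStatistic health changes, and reactivates ACDeath on EndPlay.
; Down locks all AC_Action components, disables combat and adds an overhead WI_DownMark widget.
; Undown reverses this but is not triggered here; both call CallDowns.
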(event Custom|ChangesHealth_Event
  (params (NewHealth :type Integer))
  (if (== NewHealth 0)
    (CallFunction|Down)))

(event EventBeginPlay
  (bind _asbp_character (Utilities|Casting|CastToBP_Character (Components|GetOwner)))
  (Components|Activation|Deactivate (Variables|/Game/Dynamic/Blueprints/Characters/BP_Character.BP_Character_C|GetAC_Death _asbp_character))
  (EventDispatchers|AssignChangesHealth (Variables|/Game/Dynamic/Blueprints/Characters/BP_Character.BP_Character_C|GetAC_Statistic _asbp_character) (delegate Custom|ChangesHealth_Event)))

(event EventEndPlay
  (params (EndPlayReason :type EEndPlayReason%20Enum :default "Destroyed"))
  (bind _asbp_character (Utilities|Casting|CastToBP_Character (Components|GetOwner)))
  (Components|Activation|Activate (Variables|/Game/Dynamic/Blueprints/Characters/BP_Character.BP_Character_C|GetAC_Death _asbp_character) false))

(fn Down
  (bind _asbp_character (Utilities|Casting|CastToBP_Character (Components|GetOwner)))
  (LocalVariables|SetCharacter _asbp_character)
  (Utilities|FlowControl|Sequence
    (:then_0
      (for _array_element (Actor|GetComponentsByClass (LocalVariables|GetCharacter) "/Game/Dynamic/Blueprints/Actions/AC_Action.AC_Action_C")
        (Default|Lock _array_element))
      (Default|CallDowns))
    (:then_1
      (Default|Disable (Variables|/Game/Dynamic/Blueprints/Characters/BP_Character.BP_Character_C|GetAC_Combat (LocalVariables|GetCharacter))))
    (:then_2
      (bind _returnvalue (UserInterface|CreateWidget "/Game/Dynamic/Blueprints/Death/WI_DownMark.WI_DownMark_C"))
      (bind _output_get (Variables|Default|SetDownMark _returnvalue))
      (bind _overhead (Default|GetOverHead (LocalVariables|GetCharacter)))
      (Default|AddMark _overhead _output_get))))

(fn Undown
  (bind _asbp_character (Utilities|Casting|CastToBP_Character (Components|GetOwner)))
  (LocalVariables|SetCharacter _asbp_character)
  (Utilities|FlowControl|Sequence
    (:then_0
      (for _array_element (Actor|GetComponentsByClass (LocalVariables|GetCharacter) "/Game/Dynamic/Blueprints/Actions/AC_Action.AC_Action_C")
        (Default|Unlock _array_element))
      (Default|CallDowns))
    (:then_1
      (Default|Enable (Variables|/Game/Dynamic/Blueprints/Characters/BP_Character.BP_Character_C|GetAC_Combat (LocalVariables|GetCharacter))))
    (:then_2
      (Widget|RemovefromParent (Variables|Default|GetDownMark)))))