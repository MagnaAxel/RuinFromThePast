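; Death component that destroys its owning BP_Character when health runs out.
; On BeginPlay it binds to health changes on the character's ACStatistic component.
; When health equals zero it sets IsDead, which GetIsDead exposes, waits one tick, then runs Die.
; Die destroys the owner first and only then calls the Dies event dispatcher.
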(event Custom|ChangesHealth_Event
  (params (NewHealth :type Integer))
  (if (== NewHealth 0)
    (Variables|Default|SetIsDead true)
    (Utilities|FlowControl|DelayUntilNextTick)
    (CallFunction|Die)))

(event EventBeginPlay
  (bind _asbp_character (Utilities|Casting|CastToBP_Character (Components|GetOwner)))
  (EventDispatchers|AssignChangesHealth (Variables|/Game/Dynamic/Blueprints/Characters/BP_Character.BP_Character_C|GetAC_Statistic _asbp_character) (delegate Custom|ChangesHealth_Event)))

(fn Die
  (Actor|DestroyActor (Components|GetOwner))
  (Default|CallDies))

(fn GetIsDead
  (return (Variables|Default|GetIsDead)))