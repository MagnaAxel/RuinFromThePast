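; Character component that replaces death with a downed state, deactivating ACDeath while in play and downing the owner at zero health.
; Down locks action components, disables combat and adds an overhead mark; Undown reverses these, and both fire the Downs dispatcher.
; SetUndownSequence, not called within this component, attaches an undown range actor and creates a paused timer.
; That timer runs only while undowners are present, keeping progress between pauses, then triggers Undown.
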(event Custom|ChangesHealth_Event
  (params (NewHealth :type Integer))
  (if (== NewHealth 0)
    (CallFunction|Down)))

(event EventBeginPlay
  (bind _asbp_character (Utilities|Casting|CastToBP_Character (Components|GetOwner)))
  (Components|Activation|Deactivate (Variables|/Game/Dynamic/Blueprints/Characters/BP_Character.BP_Character_C|GetAC_Death _asbp_character))
  (EventDispatchers|AssignChangesHealth (Variables|/Game/Dynamic/Blueprints/Characters/BP_Character.BP_Character_C|GetAC_Statistic _asbp_character) (delegate Custom|ChangesHealth_Event)))

(event EventEndPlay
  (params (EndPlayReason :type EEndPlayReason%20Enum :default "Destroyed"))
  (bind _asbp_character (Utilities|Casting|CastToBP_Character (Components|GetOwner)))
  (Components|Activation|Activate (Variables|/Game/Dynamic/Blueprints/Characters/BP_Character.BP_Character_C|GetAC_Death _asbp_character) false))

(event Custom|SetUndownSequence
  (bind _undownrange (CallFunction|AddUndownRange))
  (CallFunction|ListenUndownRange _undownrange)
  (bind _returnvalue (Utilities|Time|SetTimerbyEvent (delegate Custom|EndsUndownSequence_Event) 3.0))
  (bind _output_get (Variables|Default|SetUndownTimer _returnvalue))
  (Utilities|Time|PauseTimerbyHandle _output_get))

(event Custom|EndsUndownSequence_Event
  (CallFunction|Undown))

(event Custom|ListenUndownRange
  (params (UndownRange :type BP%20Undown%20Range%20Object%20Reference))
  (EventDispatchers|AssignChangesUndownerCount UndownRange (delegate Custom|ChangesUndownerCount_Event)))

(event Custom|ChangesUndownerCount_Event
  (params (UndownerCount :type Integer))
  (if (== UndownerCount 0)
    (Utilities|Time|PauseTimerbyHandle (Variables|Default|GetUndownTimer))
    (elif (== UndownerCount 1)
      (Utilities|Time|UnpauseTimerbyHandle (Variables|Default|GetUndownTimer)))))

(fn Down
  (bind _asbp_character (Utilities|Casting|CastToBP_Character (Components|GetOwner)))
  (LocalVariables|SetCharacter _asbp_character)
  (Utilities|FlowControl|Sequence
    (:then_0
      (for _array_element (Actor|GetComponentsByClass (LocalVariables|GetCharacter) "/Game/Dynamic/Blueprints/Actions/AC_Action.AC_Action_C")
        (Default|Lock _array_element))
      (Default|CallDowns))
    (:then_1
      (Default|Disable (Variables|/Game/Dynamic/Blueprints/Characters/BP_Character.BP_Character_C|GetAC_Combat (LocalVariables|GetCharacter))))
    (:then_2
      (CallFunction|AddDownMark (LocalVariables|GetCharacter)))))

(fn Undown
  (bind _asbp_character (Utilities|Casting|CastToBP_Character (Components|GetOwner)))
  (LocalVariables|SetCharacter _asbp_character)
  (Utilities|FlowControl|Sequence
    (:then_0
      (for _array_element (Actor|GetComponentsByClass (LocalVariables|GetCharacter) "/Game/Dynamic/Blueprints/Actions/AC_Action.AC_Action_C")
        (Default|Unlock _array_element))
      (Default|CallDowns))
    (:then_1
      (Default|Enable (Variables|/Game/Dynamic/Blueprints/Characters/BP_Character.BP_Character_C|GetAC_Combat (LocalVariables|GetCharacter))))
    (:then_2
      (Widget|RemovefromParent (Variables|Default|GetDownMark)))))

(fn AddUndownRange
  (bind _returnvalue (Game|SpawnActorfromClass "/Game/Dynamic/Blueprints/Death/Down/BP_UndownRange.BP_UndownRange_C" (Transformation|GetActorTransform (Components|GetOwner)) "Undefined" "MultiplyWithRoot" 0 0))
  (Transformation|AttachActorToActor _returnvalue (Components|GetOwner) "None" "SnapToTarget" "SnapToTarget" "KeepWorld" false)
  (return _returnvalue))

(fn AddDownMark
  (params (Character :type BP%20Character%20Object%20Reference) (UndownTimer :type Timer%20Handle%20Structure))
  (bind _returnvalue (UserInterface|CreateWidget "/Game/Dynamic/Blueprints/Death/Down/WI_DownMark.WI_DownMark_C" 0 UndownTimer))
  (bind _output_get (Variables|Default|SetDownMark _returnvalue))
  (bind _overhead (Default|GetOverHead Character))
  (Default|AddMark _overhead _output_get))