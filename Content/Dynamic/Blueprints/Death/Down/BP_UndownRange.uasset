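; Range actor attached to a downed character that tracks how many squadmates are close enough to undown it.
; Sphere overlaps count BP_Characters from the GameState's exploration squad, excluding the attach parent, and broadcast each change through the ChangesUndownerCount dispatcher.
; One tick after BeginPlay it binds to the parent's AC_Down Undowns event and destroys itself when that fires.
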(event OnComponentBeginOverlap(Sphere)
  (params (OverlappedComponent :type Primitive%20Component%20Object%20Reference) (OtherActor :type Actor%20Object%20Reference) (OtherComp :type Primitive%20Component%20Object%20Reference) (OtherBodyIndex :type Integer) (bFromSweep :type Boolean) (SweepResult :type Hit%20Result%20Structure%20%28by%20ref%29))
  (bind _isundowner (CallFunction|IsUndowner OtherActor))
  (if _isundowner
    (bind _result (Math|Integer|IncrementInt (Variables|Default|GetUndownerCount))
      (:%20%20
        (Default|CallChangesUndownerCount _result)))))

(event OnComponentEndOverlap(Sphere)
  (params (OverlappedComponent :type Primitive%20Component%20Object%20Reference) (OtherActor :type Actor%20Object%20Reference) (OtherComp :type Primitive%20Component%20Object%20Reference) (OtherBodyIndex :type Integer))
  (bind _isundowner (CallFunction|IsUndowner OtherActor))
  (if _isundowner
    (bind _result (Math|Integer|DecrementInt (Variables|Default|GetUndownerCount))
      (:%20%20
        (Default|CallChangesUndownerCount _result)))))

(event Custom|Undowns_Event
  (Actor|DestroyActor))

(event EventBeginPlay
  (Utilities|FlowControl|DelayUntilNextTick)
  (EventDispatchers|AssignUndowns (Actor|GetComponentbyClass (Actor|GetAttachParentActor) "/Game/Dynamic/Blueprints/Death/Down/AC_Down.AC_Down_C") (delegate Custom|Undowns_Event)))

(fn ConstructionScript)

(fn IsUndowner
  (params (Object :type Actor%20Object%20Reference))
  (bind _asbp_character (Utilities|Casting|CastToBP_Character Object))
  (bind _asgsb_default (Utilities|Casting|CastToGSB_Default (Game|GetGameState)))
  (bind _explorationsquad (Default|GetExplorationSquad _asgsb_default))
  (return (and (!= _asbp_character (Actor|GetAttachParentActor)) (Utilities|Array|ContainsItem _explorationsquad _asbp_character))))