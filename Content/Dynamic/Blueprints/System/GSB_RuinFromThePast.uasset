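; GSB_RuinFromThePast is a system Blueprint, apparently a game state, that holds the exploration squad roster.
; Its construction script finds and caches the level's BP_ExplorationSquadStart actor, reporting through DevFeedback if none exists.
; Adding a member calls AddACDown on the character, appends it to the squad array and broadcasts the AddsSquadMember dispatcher.
; A getter exposes the squad to other systems.
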(fn ConstructionScript
  (bind _returnvalue (Actor|GetActorOfClass "/Game/Dynamic/Blueprints/System/BP_ExplorationSquadStart.BP_ExplorationSquadStart_C"))
  (Utilities|IsValid _returnvalue
    (:Is%20Valid
      (Variables|Default|SetExplorationSquadStart _returnvalue))
    (:Is%20Not%20Valid
      (CallFunction|DevFeedback "NewEnumerator2" "ExplorationSquadStart not found"))))

(fn GetExplorationSquad
  (return (Variables|Default|GetExplorationSquad)))

(fn AddExplorationSquadMember
  (params (Character :type BP%20Character%20Object%20Reference%20%28by%20ref%29))
  (AddComponent|AddACDown Character)
  (Utilities|Array|Add (Variables|Default|GetExplorationSquad) Character)
  (Default|CallAddsSquadMember Character))