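; BP_ExplorationSquadStart is a placed marker that provides start points for the exploration squad.
; When BP_Eoli overlaps its sphere, it registers itself as the current ExplorationSquadStart on the GSB_RuinFromThePast game state, so the most recently entered marker replaces the previous one.
; GetOneStart maps an index to one of five capsule components that serve as the individual start spots.
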(event OnComponentBeginOverlap(Sphere)
  (params (OverlappedComponent :type Primitive%20Component%20Object%20Reference) (OtherActor :type Actor%20Object%20Reference) (OtherComp :type Primitive%20Component%20Object%20Reference) (OtherBodyIndex :type Integer) (bFromSweep :type Boolean) (SweepResult :type Hit%20Result%20Structure%20%28by%20ref%29))
  (Utilities|Casting|CastToBP_Eoli OtherActor)
  (bind _asgsb_ruin_from_the_past (Utilities|Casting|CastToGSB_RuinFromThePast (Game|GetGameState)))
  (Variables|/Game/Dynamic/Blueprints/System/GSB_RuinFromThePast.GSB_RuinFromThePast_C|SetExplorationSquadStart _asgsb_ruin_from_the_past self))

(fn ConstructionScript)

(fn GetOneStart
  (params (Index :type Integer))
  (return (Utilities|Select :Index Index :Option%200 (Variables|Default|GetCapsule0) :Option%201 (Variables|Default|GetCapsule1) :Option%202 (Variables|Default|GetCapsule2) :Option%203 (Variables|Default|GetCapsule3) :Option%204 (Variables|Default|GetCapsule4))))