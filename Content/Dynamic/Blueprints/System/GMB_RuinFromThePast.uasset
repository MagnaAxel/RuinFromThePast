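; Game mode Blueprint for RuinFromThePast that spawns the exploration squad and handles its retreat when every member is down.
; On BeginPlay it spawns the squad classes held by the game state at indexed start points and registers them there.
; It binds each added member's AC_Down event, rechecking the whole squad on every down.
; A full wipe waits a tick, teleports members to their starts, ends their down state and shows game over.
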(event EventBeginPlay
  (bind _asgsb_ruin_from_the_past (Utilities|Casting|CastToGSB_RuinFromThePast (Game|GetGameState))
    (:then
      (Variables|Default|SetGSB _asgsb_ruin_from_the_past)
      (CallFunction|ListenAddSquadMember)
      (CallFunction|SpawnExplorationSquad))
    (:CastFailed
      (CallFunction|DevFeedback "NewEnumerator2" "Game State is not GSB"))))

(event Custom|Downs_Event
  (bind _explorationsquad (Default|GetExplorationSquad (Variables|Default|GetGSB)))
  (bind (_array_element _array_index) (Utilities|Array|ForEachLoopwithBreak _explorationsquad :!label _label)
    (:LoopBody
      (bind _isdown (Default|GetIsDown (Actor|GetComponentbyClass _array_element "/Game/Dynamic/Blueprints/Death/AC_Down.AC_Down_C")))
      (if _isdown
        (if (== _array_index (Utilities|Array|LastIndex _explorationsquad))
          (Utilities|FlowControl|DelayUntilNextTick)
          (CallFunction|RetreatExplorationSquad))
        (else
          (goto _label Break))))))

(event Custom|AddsSquadMember_Event
  (params (Character :type BP%20Character%20Object%20Reference))
  (EventDispatchers|AssignDowns (Actor|GetComponentbyClass Character "/Game/Dynamic/Blueprints/Death/AC_Down.AC_Down_C") (delegate Custom|Downs_Event)))

(event Custom|ListenAddSquadMember
  (EventDispatchers|AssignAddsSquadMember (Variables|Default|GetGSB) (delegate Custom|AddsSquadMember_Event)))

(fn ConstructionScript)

(fn SpawnExplorationSquad
  (for (_array_element _array_index) (Variables|/Game/Dynamic/Blueprints/System/GSB_RuinFromThePast.GSB_RuinFromThePast_C|GetExplorationSquadClasses (Variables|Default|GetGSB))
    (bind _returnvalue (Default|GetOneStart (Variables|/Game/Dynamic/Blueprints/System/GSB_RuinFromThePast.GSB_RuinFromThePast_C|GetExplorationSquadStart (Variables|Default|GetGSB)) _array_index))
    (bind _returnvalue_2 (Game|SpawnActorfromClass _array_element (Transformation|GetWorldTransform _returnvalue) "Undefined" "MultiplyWithRoot" 0 0))
    (bind _asbp_character (Utilities|Casting|CastToBP_Character _returnvalue_2))
    (Default|AddExplorationSquadMember (Variables|Default|GetGSB) _asbp_character)))

(fn RetreatExplorationSquad
  (bind _explorationsquad (Default|GetExplorationSquad (Variables|Default|GetGSB)))
  (for (_array_element _array_index) _explorationsquad
    (bind _returnvalue (Default|GetOneStart (Variables|/Game/Dynamic/Blueprints/System/GSB_RuinFromThePast.GSB_RuinFromThePast_C|GetExplorationSquadStart (Variables|Default|GetGSB)) _array_index))
    (Transformation|SetActorTransform _array_element (Transformation|GetWorldTransform _returnvalue) false true)
    (Default|EndsUndownSequenceEvent (Actor|GetComponentbyClass _array_element "/Game/Dynamic/Blueprints/Death/AC_Down.AC_Down_C"))
    (bind _aspc_ruin_from_the_past (Utilities|Casting|CastToPC_RuinFromThePast (Game|GetPlayerController 0)))
    (bind _wi (Default|GetWI _aspc_ruin_from_the_past))
    (Default|Switch _wi (Variables|/Game/Dynamic/Blueprints/Controllers/Player/Interface/WI_RuinFromThePast.WI_RuinFromThePast_C|GetWI_GameOver _wi))))