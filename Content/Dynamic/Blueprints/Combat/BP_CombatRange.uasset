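; Combat range sensor actor attached to a BP_Character, tracking which actors are within the range of its current weapon.
; One tick after BeginPlay it gets the parent's ACAttack component, binds to its weapon change dispatcher and applies any current weapon.
; A weapon change resizes the Sphere to the weapon's Range and updates overlaps.
; Sphere begin and end overlaps are rebroadcast through the Encounters and Separates dispatchers.
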(event OnComponentBeginOverlap(Sphere)
  (params (OverlappedComponent :type Primitive%20Component%20Object%20Reference) (OtherActor :type Actor%20Object%20Reference) (OtherComp :type Primitive%20Component%20Object%20Reference) (OtherBodyIndex :type Integer) (bFromSweep :type Boolean) (SweepResult :type Hit%20Result%20Structure%20%28by%20ref%29))
  (Default|CallEncounters OtherActor))

(event OnComponentEndOverlap(Sphere)
  (params (OverlappedComponent :type Primitive%20Component%20Object%20Reference) (OtherActor :type Actor%20Object%20Reference) (OtherComp :type Primitive%20Component%20Object%20Reference) (OtherBodyIndex :type Integer))
  (Default|CallSeparates OtherActor))

(event Custom|ChangesWeapon_Event
  (params (Weapon :type BP%20Weapon%20Object%20Reference))
  (Components|Sphere|SetSphereRadius (Variables|Default|GetSphere) (Variables|/Game/Dynamic/Blueprints/Objects/Weapons/BP_Weapon.BP_Weapon_C|GetRange Weapon) true))

(event EventBeginPlay
  (Utilities|FlowControl|DelayUntilNextTick)
  (bind _asbp_character (Utilities|Casting|CastToBP_Character (Actor|GetAttachParentActor)))
  (EventDispatchers|AssignChangesWeapon (Variables|/Game/Dynamic/Blueprints/Characters/BP_Character.BP_Character_C|GetAC_Attack _asbp_character) (delegate Custom|ChangesWeapon_Event))
  (bind _weapon (Default|GetWeapon (Variables|/Game/Dynamic/Blueprints/Characters/BP_Character.BP_Character_C|GetAC_Attack _asbp_character)))
  (Utilities|IsValid _weapon
    (:Is%20Valid
      (CallFunction|ChangesWeaponEvent _weapon))))

(fn ConstructionScript)