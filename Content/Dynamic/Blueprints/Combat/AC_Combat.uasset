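; AC_Combat is a character component that tracks nearby hostile characters, combat state and the current target.
; It spawns an attached BP_CombatRange actor, whose encounter and separate events add or remove characters of enemy factions.
; The first enemy enters combat and the last removal leaves it, while a wrapping index cycles targets and broadcasts changes.
; Enable and Disable toggle the range sphere; disabling clears enemies without updating combat state.
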(event EventEndPlay
  (params (EndPlayReason :type EEndPlayReason%20Enum :default "Destroyed"))
  (Actor|DestroyActor (Variables|Default|GetCombatRange)))

(event EventBeginPlay
  (CallFunction|AddCombatRange)
  (CallFunction|ListenEncounters)
  (CallFunction|ListenSeparates))

(event Custom|ListenEncounters
  (EventDispatchers|AssignEncounters (Variables|Default|GetCombatRange) (delegate Custom|Encounters_Event)))

(event Custom|Encounters_Event
  (params (Actor :type Actor%20Object%20Reference))
  (bind _asbp_character (Utilities|Casting|CastToBP_Character Actor))
  (if (Utilities|Set|Contains (Variables|Default|GetEnemyFactions) (Variables|AC_Combat_C|GetFaction (Variables|/Game/Dynamic/Blueprints/Characters/BP_Character.BP_Character_C|GetAC_Combat _asbp_character)))
    (CallFunction|AddEnemy _asbp_character)))

(event Custom|ListenSeparates
  (EventDispatchers|AssignSeparates (Variables|Default|GetCombatRange) (delegate Custom|Separates_Event)))

(event Custom|Separates_Event
  (params (Actor :type Actor%20Object%20Reference))
  (bind _asbp_character (Utilities|Casting|CastToBP_Character Actor))
  (if (Utilities|Set|Contains (Variables|Default|GetEnemyFactions) (Variables|AC_Combat_C|GetFaction (Variables|/Game/Dynamic/Blueprints/Characters/BP_Character.BP_Character_C|GetAC_Combat _asbp_character)))
    (CallFunction|RemoveEnemy _asbp_character)))

(fn AddCombatRange
  (bind _returnvalue (Game|SpawnActorfromClass "/Game/Dynamic/Blueprints/Combat/BP_CombatRange.BP_CombatRange_C" (Transformation|GetActorTransform (Components|GetOwner)) "Undefined" "MultiplyWithRoot" 0 0))
  (bind _output_get (Variables|Default|SetCombatRange _returnvalue))
  (Transformation|AttachActorToActor _output_get (Components|GetOwner) "None" "SnapToTarget" "SnapToTarget" "KeepWorld" false))

(fn Enable
  (Components|Activation|Activate (Variables|/Game/Dynamic/Blueprints/Combat/BP_CombatRange.BP_CombatRange_C|GetSphere (Variables|Default|GetCombatRange)) false)
  (CallFunction|DevFeedback "NewEnumerator0" "Activate combat range"))

(fn Disable
  (Components|Activation|Deactivate (Variables|/Game/Dynamic/Blueprints/Combat/BP_CombatRange.BP_CombatRange_C|GetSphere (Variables|Default|GetCombatRange)))
  (Variables|Default|SetTargetIndex 0)
  (Utilities|Array|Clear (Variables|Default|GetEnemies))
  (CallFunction|DevFeedback "NewEnumerator0" "Deactivate combat range"))

(fn AddEnemy
  (params (Enemy :type BP%20Character%20Object%20Reference%20%28by%20ref%29))
  (Utilities|Array|Add (Variables|Default|GetEnemies) Enemy)
  (if (== (Utilities|Array|Length (Variables|Default|GetEnemies)) 1)
    (bind _output_get (Variables|Default|SetInCombat true))
    (Default|CallEntersCombat _output_get)
    (CallFunction|NextTargetIndex)))

(fn RemoveEnemy
  (params (Enemy :type BP%20Character%20Object%20Reference))
  (Utilities|Array|RemoveItem (Variables|Default|GetEnemies) Enemy)
  (CallFunction|SecureTargetIndex)
  (if (== (Utilities|Array|Length (Variables|Default|GetEnemies)) 0)
    (bind _output_get (Variables|Default|SetInCombat false))
    (Default|CallLeavesCombat _output_get)))

(fn NextTargetIndex
  (Math|Integer|IncrementInt (Variables|Default|GetTargetIndex)
    (:%20%20
      (CallFunction|SecureTargetIndex))))

(fn PreviousTargetIndex
  (Math|Integer|DecrementInt (Variables|Default|GetTargetIndex)
    (:%20%20
      (CallFunction|SecureTargetIndex))))

(fn SecureTargetIndex
  (Utilities|FlowControl|Sequence
    (:then_0
      (if (> (Variables|Default|GetTargetIndex) (Utilities|Array|LastIndex (Variables|Default|GetEnemies)))
        (Variables|Default|SetTargetIndex 0)))
    (:then_1
      (if (< (Variables|Default|GetTargetIndex) 0)
        (Variables|Default|SetTargetIndex (Utilities|Array|LastIndex (Variables|Default|GetEnemies)))))
    (:then_2
      (bind _target (CallFunction|GetTarget))
      (Default|CallChangesTarget _target))))

(fn GetTarget
  (return (Utilities|Array|Get(acopy) (Variables|Default|GetEnemies) (Variables|Default|GetTargetIndex))))

(fn GetinCombat
  (return (Variables|Default|GetInCombat)))