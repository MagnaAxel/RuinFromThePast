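; Actor component that shows a combat marker widget above the character's current combat target.
; On BeginPlay it casts its owner to BP_Character, creates a WI_CombatMark widget and binds to the combat component's target-change event.
; On each change it removes the widget from its parent and, if the new target is valid, adds it to that target's overhead display.
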(event Custom|ChangesTarget_Event
  (params (Target :type BP%20Character%20Object%20Reference))
  (Widget|RemovefromParent (Variables|Default|GetCombatMark))
  (Utilities|IsValid Target
    (:Is%20Valid
      (bind _overhead (Default|GetOverHead Target))
      (Default|AddMark _overhead (Variables|Default|GetCombatMark)))))

(event EventBeginPlay
  (bind _asbp_character (Utilities|Casting|CastToBP_Character (Components|GetOwner)))
  (EventDispatchers|AssignChangesTarget (Variables|/Game/Dynamic/Blueprints/Characters/BP_Character.BP_Character_C|GetAC_Combat _asbp_character) (delegate Custom|ChangesTarget_Event))
  (bind _returnvalue (UserInterface|CreateWidget "/Game/Dynamic/Blueprints/Combat/CombatMarker/WI_CombatMark.WI_CombatMark_C"))
  (Variables|Default|SetCombatMark _returnvalue))