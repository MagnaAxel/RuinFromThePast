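; AC_Locket is an actor component that manages the locket attached to its owning actor.
; SetLocket records the current locket's class and destroys it, then stores the new one and snaps it to a socket on the owner's skeletal mesh, keeping world scale.
; It returns the previous class to the caller, and GetLocket exposes the stored locket.
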(fn SetLocket
  (params (Locket :type BP%20Locket%20Object%20Reference))
  (Utilities|FlowControl|Sequence
    (:then_0
      (Utilities|IsValid (Variables|Default|GetLocket)
        (:Is%20Valid
          (LocalVariables|SetLocalPreviousLocketClass (Utilities|GetClass (Variables|Default|GetLocket)))
          (Actor|DestroyActor (Variables|Default|GetLocket)))))
    (:then_1
      (bind _output_get (Variables|Default|SetLocket Locket))
      (Transformation|AttachComponentToComponent _output_get (Actor|GetComponentbyClass (Components|GetOwner) "/Script/Engine.SkeletalMeshComponent") (Variables|Default|GetSocketName) "SnapToTarget" "SnapToTarget" "KeepWorld" false)
      (return (LocalVariables|GetLocalPreviousLocketClass)))))

(fn GetLocket
  (return (Variables|Default|GetLocket)))