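; BP_MeleeAttack is a melee weapon attack actor that moves relative to the attacking character.
; AttackMovement rotates the attack vector by the character's rotation, scales it by the weapon's final range and makes a swept move to that offset from the character's location.
; AttackUpdate runs the parent update, then orients the attack to its focus location.
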(fn ConstructionScript
  (|CallParentFunction))

(fn AttackMovement
  (params (AttackVector :type Vector :default "0, 0, 0"))
  (bind _finalrange (Default|GetFinalRange (Variables|Default|GetWeapon)))
  (Transformation|SetActorLocation (+ (* (Math|Vector|RotateVector AttackVector (Transformation|GetActorRotation (Variables|/Game/Dynamic/Blueprints/Objects/Weapons/BP_Weapon.BP_Weapon_C|GetCharacter (Variables|Default|GetWeapon)))) _finalrange) (Transformation|GetActorLocation (Variables|/Game/Dynamic/Blueprints/Objects/Weapons/BP_Weapon.BP_Weapon_C|GetCharacter (Variables|Default|GetWeapon)))) true false))

(fn AttackUpdate
  (params (AttackVector :type Vector :default "0, 0, 0"))
  (|CallParentFunction AttackVector)
  (CallFunction|OrienttoFocusLocation))