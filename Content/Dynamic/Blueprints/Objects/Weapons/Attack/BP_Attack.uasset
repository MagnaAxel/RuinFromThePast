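; Base attack actor that acts as a weapon's short-lived hitbox, turning its character toward the combat target, or straight ahead without one.
; A timeline driven by the weapon's vector curve feeds AttackMovement, an empty hook, then signals completion and destroys the actor.
; Its weapon-sized sphere hits each actor once, filters characters by enemy faction, and sends weapon damage to the actor and components implementing INT_Damage.
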(event OnComponentBeginOverlap(Sphere)
  (params (OverlappedComponent :type Primitive%20Component%20Object%20Reference) (OtherActor :type Actor%20Object%20Reference) (OtherComp :type Primitive%20Component%20Object%20Reference) (OtherBodyIndex :type Integer) (bFromSweep :type Boolean) (SweepResult :type Hit%20Result%20Structure%20%28by%20ref%29))
  (bind _isnewhit (CallFunction|IsNewHit OtherActor))
  (if _isnewhit
    (bind _isvalidhit (CallFunction|IsValidHit OtherActor))
    (if _isvalidhit
      (CallFunction|HitDamageInterfaces OtherActor))))

(event Custom|AttackSequence
  (CallFunction|ApplyFocus)
  (bind _attacktrack (Timeline|AttackTimeline PlayFromStart)
    (:Update
      (CallFunction|AttackUpdate _attacktrack))
    (:Finished
      (CallFunction|AttackFinished))))

(event EventBeginPlay
  (CallFunction|AttackSequence))

(fn ConstructionScript
  (Utilities|IsValid (Variables|Default|GetWeapon)
    (:Is%20Valid
      (Components|Sphere|SetSphereRadius (Variables|Default|GetSphere) (Variables|/Game/Dynamic/Blueprints/Objects/Weapons/BP_Weapon.BP_Weapon_C|GetSize (Variables|Default|GetWeapon)) true)
      (bind _attacktrack (Default|GetAttackTrack (Variables|Default|GetWeapon)))
      (Class|TimelineComponent|SetVectorCurve (Variables|Default|GetAttackTimeline) _attacktrack "AttackTrack")
      (Class|TimelineComponent|SetTimelineLengthMode (Variables|Default|GetAttackTimeline) "TL_LastKeyFrame"))))

(fn SetFocusLocation
  (bind _target (Default|GetTarget (Variables|/Game/Dynamic/Blueprints/Characters/BP_Character.BP_Character_C|GetAC_Combat (Variables|/Game/Dynamic/Blueprints/Objects/Weapons/BP_Weapon.BP_Weapon_C|GetCharacter (Variables|Default|GetWeapon)))))
  (Utilities|IsValid _target
    (:Is%20Valid
      (Variables|Default|SetFocusLocation (Transformation|GetActorLocation _target)))
    (:Is%20Not%20Valid
      (CallFunction|SetFrontFocusLocation))))

(fn SetFrontFocusLocation
  (bind _weapon (Variables|Default|GetWeapon))
  (bind _character (Variables|/Game/Dynamic/Blueprints/Objects/Weapons/BP_Weapon.BP_Weapon_C|GetCharacter _weapon))
  (bind _finalrange (Default|GetFinalRange (Variables|Default|GetWeapon)))
  (Variables|Default|SetFocusLocation (+ (* (Transformation|GetActorForwardVector _character) _finalrange) (Transformation|GetActorLocation _character))))

(fn OrienttoFocusLocation
  (Transformation|SetActorRotation (Variables|/Game/Dynamic/Blueprints/Objects/Weapons/BP_Weapon.BP_Weapon_C|GetCharacter (Variables|Default|GetWeapon)) (Math|Rotator|MakeRotator 0.0 0.0 (.yaw (Math|Rotator|FindLookatRotation (Transformation|GetActorLocation (Variables|/Game/Dynamic/Blueprints/Objects/Weapons/BP_Weapon.BP_Weapon_C|GetCharacter (Variables|Default|GetWeapon))) (Variables|Default|GetFocusLocation))))))

(fn ApplyFocus
  (CallFunction|SetFocusLocation)
  (CallFunction|OrienttoFocusLocation))

(fn AttackUpdate
  (params (AttackVector :type Vector))
  (CallFunction|AttackMovement AttackVector))

(fn AttackMovement
  (params (AttackVector :type Vector)))

(fn AttackFinished
  (Default|CallAttackHasFinished)
  (Actor|DestroyActor))

(fn IsNewHit
  (params (Hit :type Actor%20Object%20Reference%20%28by%20ref%29))
  (Utilities|FlowControl|Sequence
    (:then_0
      (bind _output_get (LocalVariables|SetLocalIsNewHit (not (Utilities|Set|Contains (Variables|Default|GetTargetHit) Hit))))
      (if _output_get
        (Utilities|Set|Add (Variables|Default|GetTargetHit) Hit)))
    (:then_1
      (return (LocalVariables|GetLocalIsNewHit)))))

(fn IsValidHit
  (params (Hit :type Actor%20Object%20Reference))
  (Utilities|FlowControl|Sequence
    (:then_0
      (LocalVariables|SetLocalCombat (Variables|/Game/Dynamic/Blueprints/Characters/BP_Character.BP_Character_C|GetAC_Combat (Variables|/Game/Dynamic/Blueprints/Objects/Weapons/BP_Weapon.BP_Weapon_C|GetCharacter (Variables|Default|GetWeapon)))))
    (:then_1
      (bind _asbp_character (Utilities|Casting|CastToBP_Character Hit)
        (:then
          (LocalVariables|SetLocalEnemy _asbp_character))
        (:CastFailed
          (return true))))
    (:then_2
      (return (Utilities|Set|Contains (Variables|/Game/Dynamic/Blueprints/Combat/AC_Combat.AC_Combat_C|GetEnemyFactions (LocalVariables|GetLocalCombat)) (Variables|/Game/Dynamic/Blueprints/Combat/AC_Combat.AC_Combat_C|GetFaction (Variables|/Game/Dynamic/Blueprints/Characters/BP_Character.BP_Character_C|GetAC_Combat (LocalVariables|GetLocalEnemy))))))))

(fn HitDamageInterfaces
  (params (Target :type Object%20Object%20Reference))
  (Utilities|FlowControl|Sequence
    (:then_0
      (if (Utilities|DoesObjectImplementInterface Target "/Game/Dynamic/Blueprints/Interfaces/INT_Damage.INT_Damage_C")
        (CallFunction|DealDamage Target)))
    (:then_1
      (bind _asactor (Utilities|Casting|CastToActor Target))
      (for _array_element (Class|Actor|GetComponentsbyInterface _asactor "/Game/Dynamic/Blueprints/Interfaces/INT_Damage.INT_Damage_C")
        (CallFunction|DealDamage _array_element)))))

(fn DealDamage
  (params (Target :type Object%20Object%20Reference))
  (bind _returnvalue (Default|GetFinalDamage (Variables|Default|GetWeapon)))
  (Class|INTDamage|ReceiveDamage(Message) Target _returnvalue (Variables|Default|GetWeapon)))