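; Ranged weapon attack actor that extends a parent attack class and travels out from the weapon owner.
; ApplyFocus caches the owner's transform as the start transform.
; AttackMovement rotates the attack vector by that start rotation, scales it by the weapon's final range and does a swept move to that offset from the start location.
; AttackUpdate runs the parent update then calls CallAttackHasFinished, and AttackFinished destroys the actor.
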(fn ConstructionScript
  (|CallParentFunction))

(fn AttackMovement
  (params (AttackVector :type Vector :default "0, 0, 0"))
  (bind _finalrange (Default|GetFinalRange (Variables|Default|GetWeapon)))
  (Transformation|SetActorLocation (+ (* (Math|Vector|RotateVector AttackVector (.rotation (Variables|Default|GetStartTransform))) _finalrange) (.location (Variables|Default|GetStartTransform))) true false))

(fn AttackUpdate
  (params (AttackVector :type Vector :default "0, 0, 0"))
  (|CallParentFunction AttackVector)
  (Default|CallAttackHasFinished))

(fn AttackFinished
  (Actor|DestroyActor))

(fn ApplyFocus
  (|CallParentFunction)
  (Variables|Default|SetStartTransform (Transformation|GetActorTransform (Components|GetOwner (Variables|Default|GetWeapon)))))