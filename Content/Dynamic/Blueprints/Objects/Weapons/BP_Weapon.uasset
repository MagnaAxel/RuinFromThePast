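; BP_Weapon is a weapon Blueprint that runs attacks and tracks combo progress.
; Attack spawns an AttackType actor at the owner's transform and waits for its finished event, which advances the combo and signals completion.
; The combo index selects from AttackTracks, wrapping after the last or resetting on a timer that each new attack cancels.
; Helpers compute damage scaled by the owning BP_Character's strength, and range minus size.
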(event Custom|Attack
  (CallFunction|CancelComboReset)
  (bind _returnvalue (Game|SpawnActorfromClass (Variables|Default|GetAttackType) (Transformation|GetActorTransform (Components|GetOwner)) "Undefined" "MultiplyWithRoot" 0 self 0))
  (EventDispatchers|AssignAttackHasFinished _returnvalue (delegate Custom|AttackHasFinished_Event)))

(event Custom|AttackHasFinished_Event
  (CallFunction|IncrementCombo)
  (Default|CallHasFinishedAttacking))

(event Custom|PlayComboReset
  (Utilities|Time|SetTimerbyEvent (delegate Custom|ResetCombo) (+ (Variables|Default|GetAttackDelay) (Variables|Default|GetComboDelay))))

(event Custom|CancelComboReset
  (Utilities|Time|ClearandInvalidateTimerbyHandle (Variables|Default|GetComboTimer)))

(event Custom|ResetCombo
  (Variables|Default|SetAttackTrackIndex 0))

(event Custom|IncrementCombo
  (bind _result (Math|Integer|IncrementInt (Variables|Default|GetAttackTrackIndex))
    (:%20%20
      (if (> _result (Utilities|Array|LastIndex (Variables|Default|GetAttackTracks)))
        (Variables|Default|SetAttackTrackIndex 0)
        (else
          (CallFunction|PlayComboReset))))))

(fn ConstructionScript)

(fn GetFinalDamage
  (bind _asbp_character (Utilities|Casting|CastToBP_Character (Components|GetOwner)))
  (return (Math|Float|Truncate (* (Variables|Default|GetDamage) (Variables|/Game/Dynamic/Blueprints/Statistic/AC_Statistic.AC_Statistic_C|GetStrengthFactor (Variables|/Game/Dynamic/Blueprints/Characters/BP_Character.BP_Character_C|GetAC_Statistic _asbp_character))))))

(fn GetFinalRange
  (return (- (Variables|Default|GetRange) (Variables|Default|GetSize))))

(fn GetAttackTrack
  (return (Utilities|Array|Get(acopy) (Variables|Default|GetAttackTracks) (Variables|Default|GetAttackTrackIndex))))