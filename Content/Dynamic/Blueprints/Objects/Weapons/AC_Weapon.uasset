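; AC_Weapon is a component that stores and exposes its owner's weapon.
; SetWeapon stores the weapon through SetObject, then has the combat range from the owner's AC_Combat component refresh its radius, logging developer feedback if that component is missing.
; GetWeapon returns the stored object cast to BP_Weapon.
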(fn SetWeapon
  (params (Weapon :type BP%20Weapon%20Class%20Reference))
  (bind _returnvalue (Components|GetOwner))
  (bind _returnvalue_2 (Actor|GetComponentbyClass _returnvalue "/Game/Dynamic/Blueprints/Combat/AC_Combat.AC_Combat_C"))
  (bind _previousobjectclass (CallFunction|SetObject Weapon))
  (Utilities|IsValid _returnvalue_2
    (:Is%20Valid
      (bind _combatrange (Default|GetCombatRange _returnvalue_2))
      (Default|SetCombatRangeRadius _combatrange)
      (return _previousobjectclass))
    (:Is%20Not%20Valid
      (CallFunction|DevFeedback "NewEnumerator2" "Combat Component not found")
      (return _previousobjectclass))))

(fn GetWeapon
  (bind _object (CallFunction|GetObject))
  (bind _asbp_weapon (Utilities|Casting|CastToBP_Weapon _object))
  (return _asbp_weapon))