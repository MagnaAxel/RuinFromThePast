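; BP_Food is a food object that restores health to the BP_Character that owns it.
; Eat starts a timer for the consumption delay and broadcasts Consumes with its handle.
; When the timer fires, Regnerate adds health through the owner's ACStatistic component and broadcasts Regenerates.
; The amount is the base Regeneration plus the owner's constitution factor, truncated to an integer.
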(event Custom|Eat
  (bind _returnvalue (Utilities|Time|SetTimerbyEvent (delegate Custom|Regnerate) (Variables|Default|GetConsumptionDelay)))
  (bind _output_get (Variables|Default|SetConsumptionTimer _returnvalue))
  (Default|CallComsumes _output_get))

(event Custom|Regnerate
  (bind _asbp_character (Utilities|Casting|CastToBP_Character (Components|GetOwner)))
  (bind _returnvalue (CallFunction|GetFinalRegeneration))
  (Default|AddHealth (Variables|/Game/Dynamic/Blueprints/Characters/BP_Character.BP_Character_C|GetAC_Statistic _asbp_character) _returnvalue)
  (Default|CallRegenerates))

(fn ConstructionScript
  (|CallParentFunction))

(fn GetFinalRegeneration
  (bind _asbp_character (Utilities|Casting|CastToBP_Character (Components|GetOwner)))
  (return (Math|Float|Truncate (+ (Variables|Default|GetRegeneration) (Variables|/Game/Dynamic/Blueprints/Statistic/AC_Statistic.AC_Statistic_C|GetConstitutionFactor (Variables|/Game/Dynamic/Blueprints/Characters/BP_Character.BP_Character_C|GetAC_Statistic _asbp_character))))))