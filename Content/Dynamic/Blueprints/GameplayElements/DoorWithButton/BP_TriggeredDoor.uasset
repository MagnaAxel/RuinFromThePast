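; Two-panel sliding door that opens when any of its linked buttons activates and closes again after a short delay.
; BeginPlay binds each button's Activated event and caches both panels' positions; activation plays a timeline that lerps them apart along X, then reverses it after the delay.
; Box extent and IsOpen-based collision are set only in the construction script; the runtime collision update is disconnected, although activation toggles IsOpen.
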(event Custom|Activated_Event
  (bind _porte_2_pos_initial_1 (Variables|Default|GetPorte%202%20Pos%20Initial_1))
  (bind _port1_pos_initial (Variables|Default|GetPort1_pos_initial))
  (Variables|Default|SetIsOpen (not (Variables|Default|GetIsOpen)))
  (bind _newtrack_0 (Timeline|Timeline PlayFromStart)
    (:Update
      (Transformation|SetRelativeLocation (Variables|Default|GetPorte1) (Math|Vector|Lerp(Vector) _port1_pos_initial (+ _port1_pos_initial "100.000000,0.000000,0.000000") _newtrack_0) false false)
      (Transformation|SetRelativeLocation (Variables|Default|GetPorte2) (Math|Vector|Lerp(Vector) _porte_2_pos_initial_1 (+ _porte_2_pos_initial_1 "-100.000000,0.000000,0.000000") _newtrack_0) false false))
    (:Finished
      (Utilities|FlowControl|Delay 5.0)
      (CallFunction|Fermeture))))

(event Custom|fermeture
  (bind _porte_2_pos_initial_1 (Variables|Default|GetPorte%202%20Pos%20Initial_1))
  (bind _port1_pos_initial (Variables|Default|GetPort1_pos_initial))
  (bind _newtrack_0 (Timeline|Timeline Reverse)
    (:Update
      (Transformation|SetRelativeLocation (Variables|Default|GetPorte1) (Math|Vector|Lerp(Vector) _port1_pos_initial (+ _port1_pos_initial "100.000000,0.000000,0.000000") _newtrack_0) false false)
      (Transformation|SetRelativeLocation (Variables|Default|GetPorte2) (Math|Vector|Lerp(Vector) _porte_2_pos_initial_1 (+ _porte_2_pos_initial_1 "-100.000000,0.000000,0.000000") _newtrack_0) false false))
    (:Finished
      (Utilities|FlowControl|Delay 5.0)
      (CallFunction|Fermeture))))

(event EventBeginPlay
  (for _array_element (Variables|Default|GetButton)
    (EventDispatchers|AssignActivated _array_element (delegate Custom|Activated_Event))
    (Variables|Default|SetPort1_pos_initial (Variables|/Script/Engine.SceneComponent|GetRelativeLocation (Variables|Default|GetPorte1)))
    (Variables|Default|SetPorte%202%20Pos%20Initial_1 (Variables|/Script/Engine.SceneComponent|GetRelativeLocation (Variables|Default|GetPorte2)))))

(fn ConstructionScript
  (Components|Box|SetBoxExtent (Variables|Default|GetBox) (Variables|Default|GetIn%20Box%20Extent) true)
  (Collision|SetCollisionResponsetoAllChannels (Variables|Default|GetBox) (select (Variables|Default|GetIsOpen) "ECR_Ignore" "ECR_Block")))