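; BP_Breakable is a breakable gameplay actor that is destroyed when its integrity runs out.
; A Damage event subtracts from Integrity, while a Box hit by an actor performing an AC_Dash sets it straight to zero.
; Both routes go through SetIntegrity, which clamps at zero and destroys the actor a tick later.
; The construction script applies the Mesh variable to its skeletal mesh component.
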(event OnComponentHit(Box)
  (params (HitComponent :type Primitive%20Component%20Object%20Reference) (OtherActor :type Actor%20Object%20Reference) (OtherComp :type Primitive%20Component%20Object%20Reference) (NormalImpulse :type Vector :default "0, 0, 0") (Hit :type Hit%20Result%20Structure%20%28by%20ref%29))
  (bind _returnvalue (Actor|GetComponentbyClass OtherActor "/Game/Dynamic/Blueprints/Actions/Instances/AC_Dash.AC_Dash_C"))
  (Utilities|IsValid _returnvalue
    (:Is%20Valid
      (bind _perform (Default|GetIsPerform _returnvalue))
      (if _perform
        (CallFunction|SetIntegrity)))))

(event Custom|SetIntegrity
  (params (Integrity :type Integer))
  (bind _output_get (Variables|Default|SetIntegrity (Math|Integer|Max(Integer) Integrity)))
  (if (== _output_get 0)
    (Utilities|FlowControl|DelayUntilNextTick)
    (Actor|DestroyActor)))

(event EventDamage
  (params (Damage :type Integer%20%28by%20ref%29) (Emitter :type BP%20Weapon%20Object%20Reference))
  (CallFunction|SetIntegrity (- (Variables|Default|GetIntegrity) Damage)))

(fn ConstructionScript
  (Components|SkeletalMesh|SetSkeletalMeshAsset (Variables|Default|GetSkeletalMesh) (Variables|Default|GetMesh)))