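; Breakable wall built on a Geometry Collection that shatters when a BP_Attack actor overlaps it.
; The overlap sets UseBomb on a child FS_BombField_Prototype field actor, then sets it again after a short delay and disables collision on the box and wall pieces.
; Debug strings print at each stage, and the Break_Wall event is an empty stub.
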(event Custom|Break_Wall)

(event EventBeginPlay)

(event Collision|EventActorBeginOverlap
  (params (OtherActor :type Actor%20Object%20Reference))
  (Utilities|Casting|CastToBP_Attack OtherActor)
  (Development|PrintString "Hello")
  (bind _asfs_bomb_field_prototype (Utilities|Casting|CastToFS_BombField_Prototype (Variables|/Script/Engine.ChildActorComponent|GetChildActor (Variables|Default|GetFS_BombField_Prototype))))
  (Variables|/Engine/EditorResources/FieldNodes/FS_BombField_Prototype.FS_BombField_Prototype_C|SetuseBomb _asfs_bomb_field_prototype true)
  (Development|PrintString "Booom")
  (Utilities|FlowControl|Delay 1.0)
  (bind _asfs_bomb_field_prototype_2 (Utilities|Casting|CastToFS_BombField_Prototype (Variables|/Script/Engine.ChildActorComponent|GetChildActor (Variables|Default|GetFS_BombField_Prototype))))
  (Variables|/Engine/EditorResources/FieldNodes/FS_BombField_Prototype.FS_BombField_Prototype_C|SetuseBomb _asfs_bomb_field_prototype_2 true)
  (Collision|SetCollisionEnabled (Variables|Default|GetBox) "NoCollision")
  (Utilities|FlowControl|Delay 2.0)
  (Development|PrintString "A PLUS"))

(event EventTick
  (params (DeltaSeconds :type Float%20%28single-precision%29)))

(fn ConstructionScript)