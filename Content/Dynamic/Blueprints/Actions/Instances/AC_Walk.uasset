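; AC_Walk is an action component that moves its owning character by walking.
; On BeginPlay it sets the owner to face its movement direction instead of following controller yaw.
; Each Action call turns the 2D MovementInput into a flat world-space vector, feeds it to AddMovementInput, then runs the parent action.
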(event EventBeginPlay
  (|CallParentFunction)
  (Variables|/Script/Engine.CharacterMovementComponent|SetbOrientRotationToMovement (Variables|/Script/Engine.Character|GetCharacterMovement (Variables|Default|GetOwner)) true)
  (Variables|/Script/Engine.Pawn|SetbUseControllerRotationYaw (Variables|Default|GetOwner) false))

(event EventAction
  (Pawn|Input|AddMovementInput (Variables|Default|GetOwner) (Math|Conversions|ToVector(Vector2D) (Variables|Default|GetMovementInput)) 1.0 false)
  (|CallParentFunction))