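; Interact action component that lets its owning character interact with nearby actors.
; On BeginPlay it spawns a BP_InteractRange actor attached to the owner and binds its encounter and separate events to maintain the Interactive list.
; The action sends InteractMessage to the first listed actor, passing the owning BP_Character, and runs the parent action whether or not an interaction happens.
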(event Custom|Encounters_Event
  (params (Actor :type Actor%20Object%20Reference))
  (Utilities|Array|Add (Variables|Default|GetInteractive) Actor))

(event Custom|Separates_Event
  (params (Actor :type Actor%20Object%20Reference))
  (Utilities|Array|RemoveItem (Variables|Default|GetInteractive) Actor))

(event EventBeginPlay
  (CallFunction|AddInteractRange)
  (EventDispatchers|AssignEncounters (Variables|Default|GetInteractRange) (delegate Custom|Encounters_Event))
  (EventDispatchers|AssignSeparates (Variables|Default|GetInteractRange) (delegate Custom|Separates_Event)))

(event EventAction
  (bind _interactive (Variables|Default|GetInteractive))
  (bind _output (Utilities|Array|Get(acopy) _interactive))
  (Utilities|IsValid _output
    (:Is%20Valid
      (bind _asbp_character (Utilities|Casting|CastToBP_Character (Components|GetOwner))
        (:then
          (Class|INTInteraction|Interact(Message) _output _asbp_character)
          (|CallParentFunction))
        (:CastFailed
          (|CallParentFunction :!label _label))))
    (:Is%20Not%20Valid
      (goto _label))))

(fn AddInteractRange
  (bind _returnvalue (Game|SpawnActorfromClass "/Game/Dynamic/Blueprints/Actions/Instances/Interact/BP_InteractRange.BP_InteractRange_C" (Transformation|GetActorTransform (Components|GetOwner)) "Undefined" "MultiplyWithRoot" 0 0))
  (bind _output_get (Variables|Default|SetInteractRange _returnvalue))
  (Transformation|AttachActorToActor _output_get (Components|GetOwner) "None" "SnapToTarget" "SnapToTarget" "KeepWorld" false))