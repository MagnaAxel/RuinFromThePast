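; AC_Attack is an action component that performs its owner's attack through an equipped weapon actor.
; On BeginPlay it spawns the initial weapon, and SetWeapon replaces any existing one, attaches it to a skeletal mesh socket and broadcasts the change.
; Attacking requires a valid weapon and locks actions until the weapon signals completion.
; EndAction plays the cooldown, derived from weapon delay and character agility, then releases the locks.
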(event EventBeginPlay
  (CallFunction|InitWeapon))

(event Custom|HandleFinishedAttacking
  (EventDispatchers|UnbindEventfromHasFinishedAttacking (Variables|Default|GetWeapon) (delegate Custom|HandleFinishedAttacking))
  (|CallParentFunction))

(event EventAction
  (CallFunction|LockAction)
  (CallFunction|LockOtherActions)
  (EventDispatchers|BindEventtoHasFinishedAttacking (Variables|Default|GetWeapon) (delegate Custom|HandleFinishedAttacking))
  (Default|Attack (Variables|Default|GetWeapon)))

(fn TryAction
  (Utilities|IsValid (Variables|Default|GetWeapon)
    (:Is%20Valid
      (bind _success (|CallParentFunction))
      (return _success))))

(fn EndAction
  (CallFunction|PlayCooldown)
  (CallFunction|UnlockAction)
  (CallFunction|UnlockOtherActions)
  (|CallParentFunction))

(fn GetFinalCooldown
  (bind _asbp_character (Utilities|Casting|CastToBP_Character (Components|GetOwner))
    (:then
      (return (/ (Variables|/Game/Dynamic/Blueprints/Objects/Weapons/BP_Weapon.BP_Weapon_C|GetAttackDelay (Variables|Default|GetWeapon)) (Variables|/Game/Dynamic/Blueprints/Statistic/AC_Statistic.AC_Statistic_C|GetAgilityFactor (Variables|/Game/Dynamic/Blueprints/Characters/BP_Character.BP_Character_C|GetAC_Statistic _asbp_character)))))
    (:CastFailed
      (return (Variables|/Game/Dynamic/Blueprints/Objects/Weapons/BP_Weapon.BP_Weapon_C|GetAttackDelay (Variables|Default|GetWeapon))))))

(fn SetWeapon
  (params (Weapon :type BP%20Weapon%20Object%20Reference))
  (Utilities|FlowControl|Sequence
    (:then_0
      (Utilities|IsValid (Variables|Default|GetWeapon)
        (:Is%20Valid
          (LocalVariables|SetLocalPreviousWeaponClass (Utilities|GetClass (Variables|Default|GetWeapon)))
          (Actor|DestroyActor (Variables|Default|GetWeapon)))))
    (:then_1
      (bind _output_get (Variables|Default|SetWeapon Weapon))
      (Transformation|AttachComponentToComponent _output_get (Actor|GetComponentbyClass (Components|GetOwner) "/Script/Engine.SkeletalMeshComponent") (Variables|Default|GetSocketName) "SnapToTarget" "SnapToTarget" "KeepWorld" false)
      (Default|CallChangesWeapon (Variables|Default|GetWeapon))
      (return (LocalVariables|GetLocalPreviousWeaponClass)))))

(fn GetWeapon
  (return (Variables|Default|GetWeapon)))

(fn InitWeapon
  (bind _initweaponclass (Variables|Default|GetInitWeaponClass))
  (bind _asbp_character (Utilities|Casting|CastToBP_Character (Components|GetOwner)))
  (if (Utilities|IsValidClass _initweaponclass)
    (bind _returnvalue (Game|SpawnActorfromClass _initweaponclass (Transformation|GetActorTransform _asbp_character) "Undefined" "MultiplyWithRoot" 0 0))
    (CallFunction|SetWeapon _returnvalue)))