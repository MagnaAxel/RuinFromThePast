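; AC_Dash is a character action component that performs a short forward dash.
; It locks itself and other actions, zeroes ground friction and launches the owning BP_Character along its forward vector.
; A brief timer then cuts velocity, restores friction and calls the parent action.
; On end it starts the cooldown, calls WaitToLand and unlocks actions before the parent end logic; TryAction only proceeds with a valid character.
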(event EventBeginPlay
  (bind _asbp_character (Utilities|Casting|CastToBP_Character (Components|GetOwner)))
  (Variables|Default|SetCharacter _asbp_character))

(event Custom|FinishesDash_Event
  (bind _character (Variables|Default|GetCharacter))
  (bind _charactermovement (Variables|/Script/Engine.Character|GetCharacterMovement _character))
  (Variables|/Script/Engine.MovementComponent|SetVelocity _charactermovement (* (Variables|/Script/Engine.MovementComponent|GetVelocity _charactermovement) 0.4))
  (Variables|/Script/Engine.CharacterMovementComponent|SetGroundFriction _charactermovement 8.0)
  (|CallParentFunction))

(event EventAction
  (bind _character (Variables|Default|GetCharacter))
  (CallFunction|LockAction)
  (CallFunction|LockOtherActions)
  (Variables|/Script/Engine.CharacterMovementComponent|SetGroundFriction (Variables|/Script/Engine.Character|GetCharacterMovement _character) 0.0)
  (Character|LaunchCharacter _character (* (Transformation|GetActorForwardVector _character) (Variables|Default|GetLaunchVelocity)) true false)
  (Utilities|Time|SetTimerbyEvent (delegate Custom|FinishesDash_Event) 0.2))

(fn TryAction
  (Utilities|IsValid (Variables|Default|GetCharacter)
    (:Is%20Valid
      (bind _success (|CallParentFunction))
      (return _success))))

(fn EndAction
  (CallFunction|PlayCooldown)
  (CallFunction|WaittoLand)
  (CallFunction|UnlockAction)
  (CallFunction|UnlockOtherActions)
  (|CallParentFunction))