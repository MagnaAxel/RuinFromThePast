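; AC_Eat is an action component that lets its owner eat food obtained from its AC_Food component.
; Do proceeds only when food is valid, the owner is on the ground and the cooldown is up.
; The action locks itself and other actions, takes its cooldown from the food's satiety delay, and waits for the food's finished-eating event.
; Then starts the cooldown and unlocks actions.
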(event EventBeginPlay
  (bind _owner (Variables|Default|GetOwner))
  (bind _returnvalue (Actor|GetComponentsByClass _owner "/Game/Dynamic/Blueprints/Objects/Foods/AC_Food.AC_Food_C"))
  (bind _output (Utilities|Array|Get(acopy) _returnvalue))
  (|CallParentFunction)
  (Utilities|IsValid _output
    (:Is%20Valid
      (Variables|Default|SetFoodComponent _output))
    (:Is%20Not%20Valid
      (Development|PrintString "ERROR : No Food component found"))))

(event Custom|HandleFinishedEating
  (EventDispatchers|UnbindEventfromHasFinishedEating (Variables|Default|GetFood) (delegate Custom|HandleFinishedEating))
  (|CallParentFunction))

(event EventAction
  (CallFunction|Lock)
  (CallFunction|LockOtherActions)
  (Variables|Default|SetBaseCooldown (Variables|/Game/Dynamic/Blueprints/Objects/Foods/BP_Food.BP_Food_C|GetSatietyDelay (Variables|Default|GetFood)))
  (EventDispatchers|BindEventtoHasFinishedEating (Variables|Default|GetFood) (delegate Custom|HandleFinishedEating))
  (Default|Eat (Variables|Default|GetFood)))

(fn Do
  (bind _foodcomponent (Variables|Default|GetFoodComponent))
  (Utilities|IsValid _foodcomponent
    (:Is%20Valid
      (bind _asbp_food (Default|GetFood _foodcomponent))
      (bind _output_get (Variables|Default|SetFood _asbp_food))
      (Utilities|IsValid _output_get
        (:Is%20Valid
          (bind _returnvalue (CallFunction|IsonGround))
          (if _returnvalue
            (bind _returnvalue_2 (CallFunction|IsCooldownUp))
            (if _returnvalue_2
              (|CallParentFunction))))))))

(fn Then
  (CallFunction|PlayCooldown)
  (CallFunction|Unlock)
  (CallFunction|UnlockOtherActions)
  (|CallParentFunction))