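; AC_Action is a base component for character actions, with Do starting an action only while it is unlocked and Then marking it finished.
; A counted Locker, with lock and unlock notifications, lets cooldowns, waiting to land and other actions block it independently.
; Cooldown time scales down with the owner's agility factor, and helpers can lock or unlock every other action component on the same owner.
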(event Custom|Action
  (CallFunction|Then))

(event Custom|PlayCooldown
  (bind _finalcooldown (CallFunction|GetFinalCooldown))
  (bind _returnvalue (Utilities|Time|SetTimerbyEvent (delegate Custom|ClearCooldown) _finalcooldown))
  (Variables|Default|SetCooldownTimer _returnvalue)
  (CallFunction|Lock))

(event Custom|ClearCooldown
  (Utilities|Time|ClearandInvalidateTimerbyHandle (Variables|Default|GetCooldownTimer))
  (CallFunction|Unlock))

(event Custom|HandleLand
  (params (Hit :type Hit%20Result%20Structure%20%28by%20ref%29))
  (bind _asbp_character (Utilities|Casting|CastToBP_Character (Components|GetOwner)))
  (EventDispatchers|UnbindEventfromLandedDelegate _asbp_character (delegate Custom|HandleLand))
  (CallFunction|Unlock))

(event Custom|WaitToLand
  (bind _asbp_character (Utilities|Casting|CastToBP_Character (Components|GetOwner)))
  (if (not (AI|Components|NavMovement|IsMovingonGround (Variables|/Script/Engine.Character|GetCharacterMovement _asbp_character)))
    (EventDispatchers|AssignLandedDelegate _asbp_character (delegate Custom|HandleLand))
    (CallFunction|Lock)))

(fn Do
  (bind _returnvalue (CallFunction|GetIsLock))
  (if (not _returnvalue)
    (Variables|Default|SetIsPerform true)
    (Default|CallStarts)
    (CallFunction|Action)))

(fn Then
  (Variables|Default|SetIsPerform false)
  (Default|CallFinishes (Variables|Default|GetCooldownTimer)))

(fn Lock
  (bind _result (Math|Integer|IncrementInt (Variables|Default|GetLocker))
    (:%20%20
      (if (== _result 1)
        (Default|CallLocks)))))

(fn Unlock
  (bind _result (Math|Integer|DecrementInt (Variables|Default|GetLocker))
    (:%20%20
      (if (== _result 0)
        (Default|CallUnlocks)))))

(fn LockOtherActions
  (for _array_element (Actor|GetComponentsByClass (Components|GetOwner) "AC_Action_C")
    (if (!= self _array_element)
      (CallFunction|Lock _array_element))))

(fn UnlockOtherActions
  (for _array_element (Actor|GetComponentsByClass (Components|GetOwner) "AC_Action_C")
    (if (!= self _array_element)
      (CallFunction|Unlock _array_element))))

(fn GetIsLock
  (return (> (Variables|Default|GetLocker) 0)))

(fn GetIsonGround
  (bind _asbp_character (Utilities|Casting|CastToBP_Character (Components|GetOwner))
    (:then
      (return (AI|Components|NavMovement|IsMovingonGround (Variables|/Script/Engine.Character|GetCharacterMovement _asbp_character))))
    (:CastFailed
      (return true))))

(fn GetIsPerform
  (return (Variables|Default|GetIsPerform)))

(fn GetFinalCooldown
  (bind _asbp_character (Utilities|Casting|CastToBP_Character (Components|GetOwner))
    (:then
      (return (/ (Variables|Default|GetBaseCooldown) (Variables|/Game/Dynamic/Blueprints/Statistic/AC_Statistic.AC_Statistic_C|GetAgilityFactor (Variables|/Game/Dynamic/Blueprints/Characters/BP_Character.BP_Character_C|GetAC_Statistic _asbp_character)))))
    (:CastFailed
      (return (Variables|Default|GetBaseCooldown)))))