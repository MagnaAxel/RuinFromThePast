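; Actor component that tracks an owner's Exaltation meter and switches it into a Madness state above a threshold.
; Attack starts from AC_Attack raise Exaltation using AC_Statistic's strength factor, while a one-second looping timer lowers it by resistance while positive.
; Each change broadcasts an event and re-evaluates Madness, firing enter or leave events only on transitions.
; BeginPlay adds an Exaltation widget to the first player's HUD and EndPlay clears that container.
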(event Custom|HandleAttack
  (bind _returnvalue (Components|GetOwner))
  (bind _returnvalue_2 (Actor|GetComponentbyClass _returnvalue "/Game/Dynamic/Blueprints/Statistic/AC_Statistic.AC_Statistic_C"))
  (Utilities|IsValid _returnvalue_2
    (:Is%20Valid
      (CallFunction|SetExaltation (+ (Variables|Default|GetExaltation) (+ 1 (Variables|/Game/Dynamic/Blueprints/Statistic/AC_Statistic.AC_Statistic_C|GetStrengthFactor _returnvalue_2)))))
    (:Is%20Not%20Valid
      (Development|PrintString "ERROR : Statistic Component not found" true true "(R=1.000000,G=0.000000,B=0.000000,A=1.000000)"))))

(event Custom|ListenAttack
  (bind _returnvalue (Components|GetOwner))
  (bind _returnvalue_2 (Actor|GetComponentbyClass _returnvalue "/Game/Dynamic/Blueprints/Actions/Instances/AC_Attack.AC_Attack_C"))
  (Utilities|IsValid _returnvalue_2
    (:Is%20Valid
      (EventDispatchers|AssignHasStarted _returnvalue_2 (delegate Custom|HandleAttack)))
    (:Is%20Not%20Valid
      (Development|PrintString "ERROR : No Attack Action found" true true "(R=1.000000,G=0.000000,B=0.000000,A=1.000000)"))))

(event EventBeginPlay
  (CallFunction|AddExaltationWidget)
  (CallFunction|ListenAttack))

(event EventEndPlay
  (params (EndPlayReason :type EEndPlayReason%20Enum :default "Destroyed"))
  (CallFunction|RemoveExaltationWidget))

(event Custom|PlayCalm
  (bind _returnvalue (Utilities|Time|SetTimerbyEvent (delegate Custom|Calm) 1.0 true))
  (Variables|Default|SetCalmCooldown _returnvalue))

(event Custom|Calm
  (bind _returnvalue (Components|GetOwner))
  (bind _returnvalue_2 (Actor|GetComponentbyClass _returnvalue "/Game/Dynamic/Blueprints/Statistic/AC_Statistic.AC_Statistic_C"))
  (Utilities|IsValid _returnvalue_2
    (:Is%20Valid
      (CallFunction|SetExaltation (- (Variables|Default|GetExaltation) (+ 1 (Variables|/Game/Dynamic/Blueprints/Statistic/AC_Statistic.AC_Statistic_C|GetResistanceFactor _returnvalue_2)))))
    (:Is%20Not%20Valid
      (Development|PrintString "ERROR : Statistic Component not found" true true "(R=1.000000,G=0.000000,B=0.000000,A=1.000000)"))))

(fn SetExaltation
  (params (Exaltation :type Integer))
  (Utilities|FlowControl|Sequence
    (:then_0
      (Variables|Default|SetExaltation Exaltation)
      (Default|CallExaltationHasChanged)
      (Utilities|IsValid (Actor|GetComponentbyClass (Components|GetOwner) "/Game/Dynamic/Blueprints/Statistic/AC_Statistic.AC_Statistic_C")))
    (:then_1
      (if (> (Variables|Default|GetExaltation) 0)
        (if (not (Utilities|Time|IsValidTimerHandle (Variables|Default|GetCalmCooldown)))
          (CallFunction|PlayCalm))
        (else
          (Utilities|Time|ClearandInvalidateTimerbyHandle (Variables|Default|GetCalmCooldown)))))
    (:then_2
      (CallFunction|MadnessSwitch))))

(fn GetExaltation
  (return (Variables|Default|GetExaltation)))

(fn MadnessSwitch
  (bind _exaltation (CallFunction|GetExaltation))
  (if (> _exaltation (Variables|Default|GetTreshold))
    (if (not (Variables|Default|GetMadness))
      (Variables|Default|SetMadness true)
      (Default|CallEntersMadness))
    (elif (Variables|Default|GetMadness)
      (Variables|Default|SetMadness false)
      (Default|CallLeavesMadness))))

(fn IsMad
  (return (Variables|Default|GetMadness)))

(fn AddExaltationWidget
  (bind _aspc (Utilities|Casting|CastToPC (Game|GetPlayerController 0)))
  (bind _interface (Default|GetInterface _aspc))
  (bind _returnvalue (UserInterface|CreateWidget "/Game/Dynamic/Blueprints/Controllers/Player/Interface/HeadUpDisplay/Components/WI_Exaltation.WI_Exaltation_C" (Game|GetPlayerController 0)))
  (Widget|Panel|AddChild (Variables|/Game/Dynamic/Blueprints/Controllers/Player/Interface/HeadUpDisplay/WI_HeadUpDisplay.WI_HeadUpDisplay_C|GetHorizontalBox_Exaltation (Variables|/Game/Dynamic/Blueprints/Controllers/Player/Interface/WI_Interface.WI_Interface_C|GetWI_HeadUpDisplay _interface)) _returnvalue))

(fn RemoveExaltationWidget
  (bind _aspc (Utilities|Casting|CastToPC (Game|GetPlayerController 0)))
  (bind _interface (Default|GetInterface _aspc))
  (Widget|Panel|ClearChildren (Variables|/Game/Dynamic/Blueprints/Controllers/Player/Interface/HeadUpDisplay/WI_HeadUpDisplay.WI_HeadUpDisplay_C|GetHorizontalBox_Exaltation (Variables|/Game/Dynamic/Blueprints/Controllers/Player/Interface/WI_Interface.WI_Interface_C|GetWI_HeadUpDisplay _interface))))