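; BP_Breakable is an obstacle actor that breaks when its integrity runs out or a fast-moving character hits it.
; A Box hit by a Character moving above RequiredSpeed sets integrity straight to zero.
; Damage events instead subtract from integrity, clamped at zero.
; Both paths go through SetIntegrity, which prints the new value and destroys the actor at zero.
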(event OnComponentHit(Box)
  (params (HitComponent :type Primitive%20Component%20Object%20Reference) (OtherActor :type Actor%20Object%20Reference) (OtherComp :type Primitive%20Component%20Object%20Reference) (NormalImpulse :type Vector :default "0, 0, 0") (Hit :type Hit%20Result%20Structure%20%28by%20ref%29))
  (bind _ascharacter (Utilities|Casting|CastToCharacter OtherActor))
  (if (> (Math|Vector|VectorLength (Transformation|GetVelocity _ascharacter)) (Variables|Default|GetRequiredSpeed))
    (CallFunction|SetIntegrity)))

(event EventDamage
  (params (Damage :type Integer%20%28by%20ref%29))
  (CallFunction|SubstractIntegrity Damage))

(fn ConstructionScript)

(fn SetIntegrity
  (params (Integrity :type Integer))
  (bind _output_get (Variables|Default|SetIntegrity Integrity))
  (Development|PrintString (Utilities|String|ToString(Integer) _output_get))
  (if (== _output_get 0)
    (Actor|DestroyActor)))

(fn SubstractIntegrity
  (params (Integrity :type Integer))
  (CallFunction|SetIntegrity (Math|Integer|Max(Integer) (- (Variables|Default|GetIntegrity) Integrity))))